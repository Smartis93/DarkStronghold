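; BP_spinning_Log is a spinning log trap built from a Cylinder and a RotatingMovement component.
; On BeginPlay it stores the cylinder's world rotation and activates the rotating movement.
; Its DeactivateSpin event stops the movement and sweeps the cylinder back to the stored starting rotation.
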(event Custom|Deactivate%20Spin
  (Components|Activation|Deactivate (Variables|Default|GetRotatingMovement))
  (Transformation|SetWorldRotation (Variables|Default|GetCylinder) (Variables|Default|GetStartRotation) true false))

(event EventBeginPlay
  (Variables|Default|SetStartRotation (Transformation|GetWorldRotation (Variables|Default|GetCylinder)))
  (Components|Activation|Activate (Variables|Default|GetRotatingMovement) false))

(fn ConstructionScript)