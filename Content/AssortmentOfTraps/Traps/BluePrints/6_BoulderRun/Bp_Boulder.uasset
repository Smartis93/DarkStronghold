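; Boulder trap actor that drops or rolls a physics boulder and kills the player on contact.
; It stays frozen until ActivateBoulderTrap enables physics simulation, and ResetBoulder freezes it and teleports it back to the location saved at BeginPlay.
; CollisionSphere overlap calls PlayerDead on BP_PlayerTesi regardless of speed.
; The velocity-based death or damage check is disconnected and only prints debug strings.
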(event OnComponentBeginOverlap(CollisionSphere)
  (params (OverlappedComponent :type Primitive%20Component%20Object%20Reference) (OtherActor :type Actor%20Object%20Reference) (OtherComp :type Primitive%20Component%20Object%20Reference) (OtherBodyIndex :type Integer) (bFromSweep :type Boolean) (SweepResult :type Hit%20Result%20Structure%20%28by%20ref%29))
  ;[1 1 1] checks if player and boulder is moving fast enough to kill or just damage
  (bind _asbp_player_tesi (Utilities|Casting|CastToBP_PlayerTesi OtherActor))
  (Default|PlayerDead _asbp_player_tesi))

(event Custom|ActivateBoulderTrap
  (Physics|SetSimulatePhysics (Variables|Default|GetBoulder) true))

(event Custom|ResetBoulder
  (bind _boulder (Variables|Default|GetBoulder))
  (Physics|SetSimulatePhysics _boulder false)
  (Transformation|SetWorldLocation _boulder (Variables|Default|GetStartLocation) false true))

(event EventBeginPlay
  (Physics|SetSimulatePhysics (Variables|Default|GetBoulder) false)
  (Variables|Default|SetStartLocation (Transformation|GetWorldLocation (Variables|Default|GetBoulder))))

(event Collision|EventActorBeginOverlap
  (params (OtherActor :type Actor%20Object%20Reference)))

(fn ConstructionScript)