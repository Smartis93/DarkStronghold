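; Player input buffer component that stores an attack type entered during a buffer window.
; Open and close events toggle CanBuffer, which gates both the BufferingInput event and the equivalent SetBufferAttackType function.
; Buffering sets the AreBuffer flag and saves the attack type, which GetBuffetAttackType returns.
; ClearBuffer resets only the flag, leaving the last stored type in place.
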(event Custom|OpenBufferWindow
  (Variables|Default|SetbCanBuffer true))

(event Custom|CloseBufferWindow
  (Variables|Default|SetbCanBuffer false))

(event Custom|BufferingInput
  (params (AttackTypeBuffering :type S_AttackType%20Enum :default "NewEnumerator0"))
  (if (Variables|Default|GetbCanBuffer)
    (Variables|Default|SetbAreBuffer true)
    (Variables|Default|SetAttackTypeBuffering AttackTypeBuffering)))

(event Custom|ClearBuffer
  (Variables|Default|SetbAreBuffer false))

(fn GetBuffetAttackType
  (return (Variables|Default|GetAttackTypeBuffering)))

(fn SetBufferAttackType
  (params (AttackTypeBuffering :type S_AttackType%20Enum :default "NewEnumerator0"))
  (if (Variables|Default|GetbCanBuffer)
    (Variables|Default|SetbAreBuffer true)
    (Variables|Default|SetAttackTypeBuffering AttackTypeBuffering)
    (return)))