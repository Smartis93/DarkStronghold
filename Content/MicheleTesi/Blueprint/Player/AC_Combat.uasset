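; Combat component that holds the equipped weapon and combat state and selects melee combo montages by attack type.
; NextComboMoveset advances the combo index, prunes combos whose next attack differs and returns the first match's montage.
; StartComboMoveset only resets the index, as its logic filling the candidate list from the weapon's moveset is disconnected.
; WeaponHitBox sphere-traces pawns between weapon sockets with debug drawing, leaving hits unused.
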(event EventBeginPlay)

(event EventTick
  (params (DeltaSeconds :type Float%20%28single-precision%29)))

(event Custom|WeaponHitBox
  (bind _weaponmesh (Variables|WeaponData|GetWeaponMesh))
  (if (Variables|Default|GetisHitBoxEnable)
    (Utilities|IsValid (Variables|WeaponData|GetWeaponMesh)
      (:Is%20Valid
        (Collision|MultiSphereTraceForObjects (Transformation|GetSocketLocation _weaponmesh "Start") (Transformation|GetSocketLocation _weaponmesh "End") 2e+01 (Utilities|Array|MakeArray "ObjectTypeQuery3") false (Utilities|Array|MakeArray (Components|GetOwner)) "ForDuration" true "(R=1.000000,G=0.000000,B=0.000000,A=1.000000)" "(R=0.000000,G=1.000000,B=0.000000,A=1.000000)" 0.2)))))

(event Custom|EquippedWeaponData
  (params (Weapon :type BP%20Weapon%20Parent%20Object%20Reference))
  (bind _output_get (Variables|WeaponData|SetWeapon Weapon))
  (Variables|WeaponData|SetWeaponMesh (Variables|/Game/MicheleTesi/Blueprint/Weapons/BP_WeaponParent.BP_WeaponParent_C|GetWeaponMesh _output_get)))

(fn HaveWeapon
  (Variables|WeaponData|GetWeapon
    (:then
      (return true))
    (:else
      (return false))))

(fn ChangeState
  (params (State :type E_CharacterState%20Enum :default "NewEnumerator0"))
  (Variables|Default|SetCurrent%20State State)
  (return))

(fn StartComboMoveset
  (params (AttackType :type EAttackType%20Enum :default "LightAttack"))
  (Variables|Default|SetComboIndex 0))

(fn NextComboMoveset
  (params (AttackType :type EAttackType%20Enum :default "LightAttack"))
  (bind _avaiable_moveset (Variables|Default|GetAvaiable%20Moveset))
  (bind _avaiable_moveset_2 (Variables|Default|GetAvaiable%20Moveset))
  (bind _avaiable_moveset_3 (Variables|Default|GetAvaiable%20Moveset))
  (if (Utilities|Enum|Equal(Enum) (Variables|Default|GetCurrent%20State) "NewEnumerator1")
    (Math|Integer|IncrementInt (Variables|Default|GetComboIndex)
      (:%20%20
        (if (Utilities|Array|IsNotEmpty _avaiable_moveset)
          (bind (_arrayindex _arrayelement) (Utilities|Array|ReverseforEachLoop _avaiable_moveset)
            (:LoopBody
              (if (<= (+ (Variables|Default|GetComboIndex) 1) (Utilities|Array|Length (.attacksequence _arrayelement)))
                (if (not (Utilities|Enum|Equal(Enum) AttackType (.attacktype (Utilities|Array|Get(acopy) (.attacksequence _arrayelement) (Variables|Default|GetComboIndex)))))
                  (Utilities|Array|RemoveItem _avaiable_moveset_2 (Utilities|Array|Get(acopy) _avaiable_moveset_2 _arrayindex) :!label _label))
                (else
                  (goto _label))))
            (:Completed
              (if (Utilities|Array|IsNotEmpty _avaiable_moveset_3)
                (Variables|Default|SetCurrent%20State "NewEnumerator1")
                ;[0.15 0.15 0.15 0.5] Debug
                (for _array_element _avaiable_moveset_3
                  (Development|PrintString (Utilities|String|ToString(Name) (.comboname _array_element))))
                (return (.animmontage (Utilities|Array|Get(acopy) (.attacksequence (Utilities|Array|Get(acopy) _avaiable_moveset_3)) (Variables|Default|GetComboIndex)))))))
          (else
            (return 0)))))
    (else
      (return 0))))