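; BP_SpecialLever is a one-use puzzle lever that teleports the BloccoPuzzle actor to a fixed height, keeping its X and Y.
; Its Trigger registers the lever as the SpecialLever on an overlapping BP_PlayerTesi and clears that reference on exit.
; ActivateSpecialPuzzleLever, which is not called within this graph, moves the block, runs the same clearing path, then destroys the Trigger to prevent re-registration.
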(event OnComponentBeginOverlap(Trigger)
  (params (OverlappedComponent :type Primitive%20Component%20Object%20Reference) (OtherActor :type Actor%20Object%20Reference) (OtherComp :type Primitive%20Component%20Object%20Reference) (OtherBodyIndex :type Integer) (bFromSweep :type Boolean) (SweepResult :type Hit%20Result%20Structure%20%28by%20ref%29))
  (bind _asbp_player_tesi (Utilities|Casting|CastToBP_PlayerTesi OtherActor))
  (Variables|/Game/MicheleTesi/Blueprint/Player/BP_PlayerTesi.BP_PlayerTesi_C|SetSpecialLever _asbp_player_tesi self))

(event OnComponentEndOverlap(Trigger)
  (params (OverlappedComponent :type Primitive%20Component%20Object%20Reference) (OtherActor :type Actor%20Object%20Reference) (OtherComp :type Primitive%20Component%20Object%20Reference) (OtherBodyIndex :type Integer))
  (bind _asbp_player_tesi (Utilities|Casting|CastToBP_PlayerTesi OtherActor))
  (Variables|/Game/MicheleTesi/Blueprint/Player/BP_PlayerTesi.BP_PlayerTesi_C|SetSpecialLever _asbp_player_tesi 0))

(event Custom|ActivateSpecialPuzzleLever
  (bind _bloccopuzzle (Variables|Default|GetBloccoPuzzle))
  (bind _returnvalue (Transformation|GetActorLocation _bloccopuzzle))
  (Transformation|SetActorLocation _bloccopuzzle (Math|Vector|MakeVector (.x _returnvalue) (.y _returnvalue) 13476.0) false true)
  (Utilities|FlowControl|Sequence
    (:then_0
      (bind _asbp_player_tesi (Utilities|Casting|CastToBP_PlayerTesi (stale OnComponentEndOverlap(Trigger) OtherActor)))
      (Variables|/Game/MicheleTesi/Blueprint/Player/BP_PlayerTesi.BP_PlayerTesi_C|SetSpecialLever _asbp_player_tesi 0))
    (:then_1
      (Components|DestroyComponent (Variables|Default|GetTrigger)))))

(event EventBeginPlay)

(event Collision|EventActorBeginOverlap
  (params (OtherActor :type Actor%20Object%20Reference)))

(event EventTick
  (params (DeltaSeconds :type Float%20%28single-precision%29)))

(fn ConstructionScript)