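; Parent weapon Blueprint that lets the player register it as a pickup candidate while it is unequipped.
; Entering PickupTrigger stores the weapon in the TempSword reference on BP_PlayerTesi.
; Leaving the trigger clears any valid TempSword, without checking that it points to this weapon.
; The EquippedWeapon event sets IsEquipped, after which both overlap handlers do nothing.
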(event OnComponentBeginOverlap(PickupTrigger)
  (params (OverlappedComponent :type Primitive%20Component%20Object%20Reference) (OtherActor :type Actor%20Object%20Reference) (OtherComp :type Primitive%20Component%20Object%20Reference) (OtherBodyIndex :type Integer) (bFromSweep :type Boolean) (SweepResult :type Hit%20Result%20Structure%20%28by%20ref%29))
  (if (not (Variables|Default|GetisEquipped))
    (bind _asbp_player_tesi (Utilities|Casting|CastToBP_PlayerTesi OtherActor))
    (Variables|/Game/MicheleTesi/Blueprint/Player/BP_PlayerTesi.BP_PlayerTesi_C|SetTemp_sword _asbp_player_tesi self)))

(event OnComponentEndOverlap(PickupTrigger)
  (params (OverlappedComponent :type Primitive%20Component%20Object%20Reference) (OtherActor :type Actor%20Object%20Reference) (OtherComp :type Primitive%20Component%20Object%20Reference) (OtherBodyIndex :type Integer))
  (if (not (Variables|Default|GetisEquipped))
    (bind _asbp_player_tesi (Utilities|Casting|CastToBP_PlayerTesi OtherActor))
    (Variables|/Game/MicheleTesi/Blueprint/Player/BP_PlayerTesi.BP_PlayerTesi_C|GetTemp_sword _asbp_player_tesi
      (:then
        (Variables|/Game/MicheleTesi/Blueprint/Player/BP_PlayerTesi.BP_PlayerTesi_C|SetTemp_sword _asbp_player_tesi 0))
      (:else))))

(event Custom|EquippedWeapon
  (Variables|Default|SetisEquipped true))

(event EventBeginPlay)

(event Collision|EventActorBeginOverlap
  (params (OtherActor :type Actor%20Object%20Reference)))

(event EventTick
  (params (DeltaSeconds :type Float%20%28single-precision%29)))

(fn ConstructionScript)