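; Elevator actor that travels between its base position and a terminal position, callable toward either end or toggled by a lever event.
; On BeginPlay it caches both world locations, destroys the Terminal marker component and applies Speed as the timeline play rate.
; The timeline lerps the Base component forward or in reverse, then flips the location flags, ignoring calls while moving.
; A trigger box registers or clears the elevator on overlapping BP_PlayerTesi characters.
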(event OnComponentBeginOverlap(Box)
  (params (OverlappedComponent :type Primitive%20Component%20Object%20Reference) (OtherActor :type Actor%20Object%20Reference) (OtherComp :type Primitive%20Component%20Object%20Reference) (OtherBodyIndex :type Integer) (bFromSweep :type Boolean) (SweepResult :type Hit%20Result%20Structure%20%28by%20ref%29))
  (bind _asbp_player_tesi (Utilities|Casting|CastToBP_PlayerTesi OtherActor))
  (Variables|/Game/MicheleTesi/Blueprint/Player/BP_PlayerTesi.BP_PlayerTesi_C|SetElevator _asbp_player_tesi self))

(event OnComponentEndOverlap(Box)
  (params (OverlappedComponent :type Primitive%20Component%20Object%20Reference) (OtherActor :type Actor%20Object%20Reference) (OtherComp :type Primitive%20Component%20Object%20Reference) (OtherBodyIndex :type Integer))
  (bind _asbp_player_tesi (Utilities|Casting|CastToBP_PlayerTesi OtherActor))
  (Variables|/Game/MicheleTesi/Blueprint/Player/BP_PlayerTesi.BP_PlayerTesi_C|SetElevator _asbp_player_tesi 0))

(event Custom|Elevator%20to%20Terminal
  (bind _base (Variables|Default|GetBase))
  (bind _baseposition (Variables|Default|GetBasePosition))
  (bind _terminalposition (Variables|Default|GetTerminalPosition))
  (if (not (Variables|Default|GetbIsMoving))
    (if (Variables|Default|GetbIs%20in%20Base)
      (Variables|Default|SetbIsMoving true)
      (bind _newtrack_0 (Timeline|ElevatorTimeline PlayFromStart)
        (:Update
          (Transformation|SetWorldLocation _base (Math|Vector|Lerp(Vector) _baseposition _terminalposition _newtrack_0) false true))
        (:Finished
          (if (and (== _newtrack_0 1.0) (not (== _newtrack_0 0.0)))
            (Transformation|SetWorldLocation _base _terminalposition false true)
            (else
              (Transformation|SetWorldLocation _base _baseposition false true)))
          (if (and (Variables|Default|GetbIs%20in%20Base) (not (Variables|Default|GetbIs%20in%20Terminal)))
            (Variables|Default|SetbIs%20in%20Base false)
            (Variables|Default|SetbIs%20in%20Terminal true)
            (else
              (Variables|Default|SetbIs%20in%20Base true)
              (Variables|Default|SetbIs%20in%20Terminal false)))
          (Variables|Default|SetbIsMoving false))))))

(event Custom|Elevator%20to%20Base
  (bind _base (Variables|Default|GetBase))
  (bind _baseposition (Variables|Default|GetBasePosition))
  (bind _terminalposition (Variables|Default|GetTerminalPosition))
  (if (not (Variables|Default|GetbIsMoving))
    (if (Variables|Default|GetbIs%20in%20Terminal)
      (Variables|Default|SetbIsMoving true)
      (bind _newtrack_0 (Timeline|ElevatorTimeline ReverseFromEnd)
        (:Update
          (Transformation|SetWorldLocation _base (Math|Vector|Lerp(Vector) _baseposition _terminalposition _newtrack_0) false true))
        (:Finished
          (if (and (== _newtrack_0 1.0) (not (== _newtrack_0 0.0)))
            (Transformation|SetWorldLocation _base _terminalposition false true)
            (else
              (Transformation|SetWorldLocation _base _baseposition false true)))
          (if (and (Variables|Default|GetbIs%20in%20Base) (not (Variables|Default|GetbIs%20in%20Terminal)))
            (Variables|Default|SetbIs%20in%20Base false)
            (Variables|Default|SetbIs%20in%20Terminal true)
            (else
              (Variables|Default|SetbIs%20in%20Base true)
              (Variables|Default|SetbIs%20in%20Terminal false)))
          (Variables|Default|SetbIsMoving false))))))

(event Custom|ElevatorLever
  (bind _base (Variables|Default|GetBase))
  (bind _baseposition (Variables|Default|GetBasePosition))
  (bind _terminalposition (Variables|Default|GetTerminalPosition))
  (if (not (Variables|Default|GetbIsMoving))
    (if (and (Variables|Default|GetbIs%20in%20Base) (not (Variables|Default|GetbIs%20in%20Terminal)))
      (Variables|Default|SetbIsMoving true)
      (bind _newtrack_0 (Timeline|ElevatorTimeline PlayFromStart)
        (:Update
          (Transformation|SetWorldLocation _base (Math|Vector|Lerp(Vector) _baseposition _terminalposition _newtrack_0) false true))
        (:Finished
          (if (and (== _newtrack_0 1.0) (not (== _newtrack_0 0.0)))
            (Transformation|SetWorldLocation _base _terminalposition false true)
            (else
              (Transformation|SetWorldLocation _base _baseposition false true)))
          (if (and (Variables|Default|GetbIs%20in%20Base) (not (Variables|Default|GetbIs%20in%20Terminal)))
            (Variables|Default|SetbIs%20in%20Base false)
            (Variables|Default|SetbIs%20in%20Terminal true)
            (else
              (Variables|Default|SetbIs%20in%20Base true)
              (Variables|Default|SetbIs%20in%20Terminal false)))
          (Variables|Default|SetbIsMoving false)))
      (else
        (Variables|Default|SetbIsMoving true)
        (Timeline|ElevatorTimeline ReverseFromEnd)))))

(event EventBeginPlay
  (Components|Timeline|SetPlayRate (Variables|Default|GetElevatorTimeline) (Variables|Default|GetSpeed))
  (Variables|Default|SetBasePosition (Transformation|GetWorldLocation (Variables|Default|GetBase)))
  (Variables|Default|SetTerminalPosition (Transformation|GetWorldLocation (Variables|Default|GetTerminal)))
  (Components|DestroyComponent (Variables|Default|GetTerminal)))

(fn ConstructionScript)