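; BP_ElevatorLever is a lever actor that sends a linked elevator to one of its two ends.
; Its box overlap registers the lever on BP_PlayerTesi as the current ElevatorLever and clears that reference when the player leaves.
; LeverActivate, not called within this Blueprint, checks that the Elevator reference is valid and calls ElevatorToBase or ElevatorToTerminal depending on the IsBase flag.
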(event OnComponentBeginOverlap(Box)
  (params (OverlappedComponent :type Primitive%20Component%20Object%20Reference) (OtherActor :type Actor%20Object%20Reference) (OtherComp :type Primitive%20Component%20Object%20Reference) (OtherBodyIndex :type Integer) (bFromSweep :type Boolean) (SweepResult :type Hit%20Result%20Structure%20%28by%20ref%29))
  (bind _asbp_player_tesi (Utilities|Casting|CastToBP_PlayerTesi OtherActor))
  (Variables|/Game/MicheleTesi/Blueprint/Player/BP_PlayerTesi.BP_PlayerTesi_C|SetElevatorLever _asbp_player_tesi self))

(event OnComponentEndOverlap(Box)
  (params (OverlappedComponent :type Primitive%20Component%20Object%20Reference) (OtherActor :type Actor%20Object%20Reference) (OtherComp :type Primitive%20Component%20Object%20Reference) (OtherBodyIndex :type Integer))
  (bind _asbp_player_tesi (Utilities|Casting|CastToBP_PlayerTesi OtherActor))
  (Variables|/Game/MicheleTesi/Blueprint/Player/BP_PlayerTesi.BP_PlayerTesi_C|SetElevatorLever _asbp_player_tesi 0))

(event Custom|LeverActivate
  (if (Variables|Default|GetbIsBase)
    (bind _elevator (Variables|Default|GetElevator)
      (:then
        (Default|ElevatortoBase _elevator))
      (:else))
    (else
      (bind _elevator_2 (Variables|Default|GetElevator)
        (:then
          (Default|ElevatortoTerminal _elevator_2))
        (:else)))))

(event EventBeginPlay)

(event Collision|EventActorBeginOverlap
  (params (OtherActor :type Actor%20Object%20Reference)))

(event EventTick
  (params (DeltaSeconds :type Float%20%28single-precision%29)))

(fn ConstructionScript)