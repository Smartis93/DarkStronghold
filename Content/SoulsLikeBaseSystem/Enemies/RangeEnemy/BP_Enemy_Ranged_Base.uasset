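; Base Blueprint for ranged enemies in the Souls-like system, extending a parent enemy class with a shooting attack.
; On BeginPlay it equips the enemy's main weapon at the configured socket.
; Attack plays the shoot montage, and its notify makes the attack component fire a bullet from the weapon toward the target using the weapon's damage info.
; Montage completion or interruption both end the attack.
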(event EventBeginPlay
  (|CallParentFunction)
  (CallFunction|EquipWeaponBPI))

(event EventEquipWeaponBPI
  ;[1 1 1] Equip Weapon
  (CallFunction|EquipMainWeaponsFunc (Variables|Default|GetEnemyMainWeapon) (Variables|Default|GetMainWeaponSocketName)))

(event EventAttack
  (params (AttackTarget :type Actor%20Object%20Reference))
  ;[1 1 1] Attack
  (|CallParentFunction AttackTarget)
  (bind _notifyname (Animation|Montage|PlayMontage (Variables|Character|GetMesh) (Variables|Init|Montage|GetRangeShootMontage))
    (:OnCompleted
      (CallFunction|AttackEnd AttackTarget :!label _label))
    (:OnInterrupted
      (goto _label))
    (:OnNotifyBegin
      (switch name _notifyname
        (:Fire
          (bind _mainweapon (CallFunction|GetMainWeapon))
          (Utilities|IsValid _mainweapon
            (:Is%20Valid
              (Default|FireBullet (Variables|Default|GetAC_AttackComponent) (Transformation|GetActorLocation _mainweapon) (Transformation|GetActorLocation AttackTarget) (.DamageInfo (CallFunction|GetMainWeaponInfo))))))))))

(fn ConstructionScript
  (|CallParentFunction))