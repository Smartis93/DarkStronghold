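; Base mage enemy that equips its weapon on BeginPlay and exposes attack, teleport and heal events.
; Ground smash, basic spell and barrage attacks go through ACAttackComponent using montages and main-weapon damage.
; Teleport is a fast, invisible flying AIMoveTo that ignores pawn collision, with VFX, then restores walking and fires OnTeleportEnd.
; Healing plays a montage, spawns a traced AOE actor that heals the mage on overlap ticks, and destroys it afterward.
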(event Custom|Teleport
  (params (Location :type Vector))
  (bind _charactermovement (Variables|Character|GetCharacterMovement))
  ;[1 1 1] Teleport Start
  (if (not (Variables|Default|GetIsTeleporting))
    (Variables|Default|SetIsTeleporting true)
    (Pawn|Components|CharacterMovement|SetMovementMode _charactermovement "MOVE_Flying" 0)
    (Variables|/Script/Engine.CharacterMovementComponent|SetMaxFlySpeed _charactermovement 5e+03)
    (Variables|/Script/Engine.CharacterMovementComponent|SetMaxAcceleration _charactermovement 99999.0)
    (Rendering|SetVisibility (Variables|Character|GetMesh) false false)
    (Collision|SetCollisionResponsetoChannel (Variables|Default|GetCapsuleComponent) "ECC_Pawn" "ECR_Ignore")
    (bind _returnvalue (Niagara|SpawnSystemAttached (Variables|Init|VFX|GetTeleportVFX) (Variables|Character|GetMesh) (Variables|Default|GetSpineSocketName) "0, 0, 0" "0, 0, 0" "KeepRelativeOffset" false))
    (Variables|Default|SetTeleportBodyEffect _returnvalue)
    (bind _returnvalue_2 (Niagara|SpawnSystemAttached (Variables|Init|VFX|GetTeleportStartTrailVFX) (Variables|Character|GetMesh) (Variables|Default|GetSpineSocketName) "0, 0, 0" "0, 0, 0" "KeepRelativeOffset" false))
    (Variables|Default|SetTeleportTrailEffect _returnvalue_2)
    (Audio|PlaySoundatLocation (Variables|Init|Sound|GetTeleportSound) "0, 0, 0" "0, 0, 0" 1.0 1.0 0.0 0 0 0 0)
    (Animation|StopAnimMontage 0)
    (AI|AIMoveTo self Location 0 15.0 false
      (:OnSuccess
        _)
      (:OnFail
        _))
    (CallFunction|TeleportEnd)
    (else
      (Utilities|FlowControl|DelayUntilNextTick)
      (Default|CallOnTeleportEnd))))

(event Custom|TeleportEnd
  (bind _charactermovement (Variables|Character|GetCharacterMovement))
  ;[1 1 1] Teleport End
  (Components|Movement|StopMovementImmediately (Variables|Character|GetCharacterMovement))
  (Pawn|Components|CharacterMovement|SetMovementMode _charactermovement "MOVE_Walking" 0)
  (Variables|/Script/Engine.CharacterMovementComponent|SetMaxAcceleration _charactermovement 1.5e+03)
  (Rendering|SetVisibility (Variables|Character|GetMesh) true false)
  (Collision|SetCollisionResponsetoChannel (Variables|Default|GetCapsuleComponent) "ECC_Pawn" "ECR_Block")
  (Default|CallOnTeleportEnd)
  (Utilities|FlowControl|Delay 0.5)
  (Variables|Default|SetIsTeleporting false)
  (Utilities|FlowControl|Sequence
    (:then_0
      (bind _teleportbodyeffect (Variables|Default|GetTeleportBodyEffect)
        (:then
          (Components|DestroyComponent _teleportbodyeffect))
        (:else)))
    (:then_1
      (bind _teleporttraileffect (Variables|Default|GetTeleportTrailEffect)
        (:then
          (Components|DestroyComponent _teleporttraileffect))
        (:else)))))

(event Custom|HealOverTime
  (params (HealEveryTimePercent :type Float%20%28double-precision%29))
  (bind _returnvalue (Transformation|GetActorLocation))
  ;[1 1 1] Heal
  (Animation|Montage|PlayMontage (Variables|Character|GetMesh) (Variables|Init|Montage|GetHeal_Montage)
    (:then
      (bind (_outhit _returnvalue_2) (Collision|LineTraceByChannel _returnvalue (* _returnvalue "1.000000,1.000000,-1000.000000") "TraceTypeQuery1" false 0 "None"))
      (if _returnvalue_2
        (bind _returnvalue_3 (Game|SpawnActorfromClass (Variables|Init|GetHealAOEActor) (Math|Transform|MakeTransform (.Location (Collision|BreakHitResult _outhit)) "0, 0, 0" "1.000000,1.000000,1.000000") "Undefined" "MultiplyWithRoot" 0 1.0 6.0 false false "ForDuration" 0))
        (bind _output_get (Variables|Init|SetHealAOERef _returnvalue_3))
        (EventDispatchers|AssignOnAoeOverlapActor _output_get (delegate Custom|OnHealTick))
        (else
          (Animation|StopAnimMontage 0))))
    (:OnCompleted
      (CallFunction|HealOverTimeEnd :!label _label))
    (:OnInterrupted
      (goto _label))))

(event Custom|HealOverTimeEnd
  ;[1 1 1] Heal
  ;;[1 1 1] HealEnd
  (Default|CallOnHealOverTimeEnd)
  (bind _healaoeref (Variables|Init|GetHealAOERef)
    (:then
      (Actor|DestroyActor _healaoeref))
    (:else)))

(event Custom|OnHealTick
  (params (Actor :type Actor%20Object%20Reference) (Hit%20Result :type Hit%20Result%20Structure))
  (bind _ac_statscomponent (Variables|Default|GetAC_StatsComponent))
  ;[1 1 1] Heal
  (if (== Actor self)
    (CallFunction|Heal (* (Default|GetMaxStats (Variables|Default|GetAC_StatsComponent) "NewEnumerator1") (stale Custom|HealOverTime HealEveryTimePercent)))
    (Default|UpdateHealthBar (Variables|Default|GetWidgetHealthBar) (Default|GetCurrentStats _ac_statscomponent "NewEnumerator1") (Default|GetMaxStats _ac_statscomponent "NewEnumerator1"))))

(event Custom|BasicAttack
  (params (AttackTarget :type Actor%20Object%20Reference))
  ;[1 1 1] Attack
  (Default|BasicMagicSpell (Variables|Default|GetAC_AttackComponent) (Utilities|Struct|MakeS_AttackInfo AttackTarget (Variables|Init|Montage|GetBasicMagicAttack_Montage) (.DamageInfo (CallFunction|GetMainWeaponInfo))) (Variables|Init|GetMagicBasicAttackProjectile)))

(event Custom|BarrageAttack
  (params (AttackTarget :type Actor%20Object%20Reference))
  ;[1 1 1] Attack
  (Default|BarrageMagicAttack (Variables|Default|GetAC_AttackComponent) (Utilities|Struct|MakeS_AttackInfo AttackTarget (Variables|Init|Montage|GetMagicBarrageAttack_Montage) (.DamageInfo (CallFunction|GetMainWeaponInfo))) (Variables|Init|GetMagicBarrageAttackProjectile)))

(event Custom|GroundSmashAttack
  (params (AttackTarget :type Actor%20Object%20Reference))
  ;[1 1 1] Attack
  (Default|GroundSmashAOE (Variables|Default|GetAC_AttackComponent) (Utilities|Struct|MakeS_AttackInfo AttackTarget (Variables|Init|Montage|GetMagicSmashAttack_Montage) (.DamageInfo (CallFunction|GetMainWeaponInfo))) 3e+02 "0, 0, 0"))

(event EventBeginPlay
  (|CallParentFunction)
  ;[1 1 1] EquipWeapon
  (CallFunction|EquipWeaponBPI))

(event Collision|EventActorBeginOverlap
  (params (OtherActor :type Actor%20Object%20Reference)))

(event EventTick
  (params (DeltaSeconds :type Float%20%28single-precision%29)))

(event EventEquipWeaponBPI
  ;[1 1 1] Equipment
  (CallFunction|EquipMainWeaponsFunc (Variables|Default|GetEnemyMainWeapon) (Variables|Default|GetMainWeaponSocketName)))

(fn ConstructionScript
  (|CallParentFunction))