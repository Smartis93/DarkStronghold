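; Souls-like boss enemy with its own health bar widget, updated on damage and cleared from the player HUD after death.
; Attack events use the attack component or montage notifies for melee combos, AOE strikes and a homing axe throw.
; Teleport is a hidden, high-speed flying AI move with a trail effect.
; Float spawns a platform and grants invincibility; teleport, float and weapon equip signal completion through dispatchers.
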(event OnDeath(AC_DamageComponent)
  ;[1 1 1] Death
  (Variables|/Game/SoulsLikeBaseSystem/ComponentsAndSystem/Components/AttackComponent/AC_AttackSystem.AC_AttackSystem_C|SetCanDoWeaponTrace (Variables|Default|GetAC_AttackComponent) false)
  ;;[1 1 1] Death
  (CallFunction|Death)
  ;;[1 1 1] Return Attack Token
  (CallFunction|ReturnAttackToken)
  (Animation|Montage|PlayMontage (Variables|Character|GetMesh) (Variables|Default|GetDealth_Montage)
    (:then
      (Utilities|FlowControl|Delay 5.0)
      ;;[1 1 1] Destroy all Weapons
      (CallFunction|UnEquipWeaponsFunc)
      (Actor|DestroyActor)
      ;;[1 1 1] Clear Boss Health Bar
      (bind _asbp_player (Utilities|Casting|CastToBP_Player (Game|GetPlayerCharacter 0)))
      (Widget|Panel|ClearChildren (Variables|/Game/SoulsLikeBaseSystem/HUD/WBP_PlayerHud.WBP_PlayerHud_C|GetBottomVerticalBox (Variables|/Game/SoulsLikeBaseSystem/Player/BP_Player.BP_Player_C|GetPlayerHUDRef _asbp_player))))))

(event Custom|Teleport
  (params (Location :type Vector) (AttackTarget :type Actor%20Object%20Reference))
  (bind _charactermovement (Variables|Character|GetCharacterMovement))
  ;[1 1 1] Teleport start
  (if (not (Variables|Default|GetIsTeleporting))
    (Variables|Default|SetIsTeleporting true)
    (Pawn|Components|CharacterMovement|SetMovementMode _charactermovement "MOVE_Flying" 0)
    (Variables|/Script/Engine.CharacterMovementComponent|SetMaxFlySpeed _charactermovement 5e+03)
    (Variables|/Script/Engine.CharacterMovementComponent|SetMaxAcceleration _charactermovement 99999.0)
    (Rendering|SetVisibility (Variables|Character|GetMesh) false true)
    (Collision|SetCollisionResponsetoChannel (Variables|Default|GetCapsuleComponent) "ECC_Pawn" "ECR_Ignore")
    (bind _returnvalue (Niagara|SpawnSystemAttached (Variables|Init|VFX|GetTeleportStartVFX) (Variables|Character|GetMesh) (Variables|Default|GetSpineSocketName) "0, 0, 0" "0, 0, 0" "KeepRelativeOffset" false))
    (Variables|Default|SetTeleportTrailEffect _returnvalue)
    (Audio|PlaySoundatLocation (Variables|Init|Sound|GetTeleportStartSound) "0, 0, 0" "0, 0, 0" 1.0 1.0 0.0 0 0 0 0)
    (Animation|StopAnimMontage 0)
    (AI|AIMoveTo self Location AttackTarget 1.5e+02 false
      (:OnSuccess
        _)
      (:OnFail
        _))
    (CallFunction|TeleportEnd)
    (else
      (Utilities|FlowControl|DelayUntilNextTick)
      (Default|CallOnTeleportEnd))))

(event Custom|TeleportEnd
  (bind _charactermovement (Variables|Character|GetCharacterMovement))
  ;[1 1 1] Teleport end
  (Components|Movement|StopMovementImmediately (Variables|Character|GetCharacterMovement))
  (Pawn|Components|CharacterMovement|SetMovementMode _charactermovement "MOVE_Walking" 0)
  (Variables|/Script/Engine.CharacterMovementComponent|SetMaxAcceleration _charactermovement 1.5e+03)
  (Rendering|SetVisibility (Variables|Character|GetMesh) true true)
  (Collision|SetCollisionResponsetoChannel (Variables|Default|GetCapsuleComponent) "ECC_Pawn" "ECR_Block")
  (Default|CallOnTeleportEnd)
  (Utilities|FlowControl|Delay 0.5)
  (Variables|Default|SetIsTeleporting false)
  (bind _teleporttraileffect (Variables|Default|GetTeleportTrailEffect)
    (:then
      (Components|DestroyComponent _teleporttraileffect))
    (:else)))

(event Custom|StartFloat
  (bind _returnvalue (Transformation|GetActorLocation))
  ;[1 1 1] Float platform
  (Variables|/Game/SoulsLikeBaseSystem/ComponentsAndSystem/Components/DamageComponent/AC_DamageSystem.AC_DamageSystem_C|SetIsInvincible (Variables|Default|GetAC_DamageComponent) true)
  (bind (_outhit _returnvalue_2) (Collision|LineTraceByChannel _returnvalue (* _returnvalue "1.000000,1.000000,-1000.000000") "TraceTypeQuery1" false 0 "None"))
  (if _returnvalue_2
    (bind _returnvalue_3 (Game|SpawnActorfromClass "/Game/SoulsLikeBaseSystem/Enemies/Props/BP_FloatingPlatform.BP_FloatingPlatform_C" (Math|Transform|MakeTransform (.Location (Collision|BreakHitResult _outhit)) "0, 0, 0" "1.000000,1.000000,1.000000") "Undefined" "MultiplyWithRoot" 0 0))
    (bind _output_get (Variables|Default|SetFloatingPlatformRef _returnvalue_3))
    (EventDispatchers|AssignOnFloatTimelineFinished _output_get (delegate Custom|OnFloatTimelineFinished_Event))))

(event Custom|OnFloatTimelineFinished_Event
  ;[1 1 1] Float platform
  (EventDispatchers|UnbindEventfromOnFloatTimelineFinished (stale Custom|StartFloat _output_get) (delegate Custom|OnFloatTimelineFinished_Event))
  (Default|CallOnFloatReachHight))

(event Custom|StopFloat
  ;[1 1 1] Float platform
  (bind _floatingplatformref (Variables|Default|GetFloatingPlatformRef)
    (:then
      (Default|StopFloating _floatingplatformref)
      (EventDispatchers|AssignOnFloatTimelineFinished _floatingplatformref (delegate Custom|OnFloatTimelineFinished_Event_0)))
    (:else
      (Utilities|FlowControl|DelayUntilNextTick)
      (Variables|/Game/SoulsLikeBaseSystem/ComponentsAndSystem/Components/DamageComponent/AC_DamageSystem.AC_DamageSystem_C|SetIsInvincible (Variables|Default|GetAC_DamageComponent) false)
      (Actor|DestroyActor _floatingplatformref)
      (Default|CallOnFloatEnded))))

(event Custom|OnFloatTimelineFinished_Event_0
  ;[1 1 1] Float platform
  (EventDispatchers|UnbindEventfromOnFloatTimelineFinished (stale Custom|StopFloat _floatingplatformref) (delegate Custom|OnFloatTimelineFinished_Event_0))
  (Variables|/Game/SoulsLikeBaseSystem/ComponentsAndSystem/Components/DamageComponent/AC_DamageSystem.AC_DamageSystem_C|SetIsInvincible (Variables|Default|GetAC_DamageComponent) false)
  (Actor|DestroyActor (stale Custom|StopFloat _floatingplatformref))
  (Default|CallOnFloatEnded))

(event Custom|AOETrail
  (params (AttackTarget :type Actor%20Object%20Reference))
  ;[1 1 1] Attack
  ;;[1 1 1] AOE Trail
  (CallFunction|Attack AttackTarget)
  (bind _notifyname (Animation|Montage|PlayMontage (Variables|Character|GetMesh) (Variables|Init|Montage|GetAOETrail_Montage))
    (:OnCompleted
      (CallFunction|AttackEnd AttackTarget :!label _label))
    (:OnInterrupted
      (goto _label))
    (:OnNotifyBegin
      (switch name _notifyname
        (:Strike
          (bind _returnvalue (Game|SpawnActorfromClass "/Game/SoulsLikeBaseSystem/ComponentsAndSystem/AOESystem/AOE_Blast/BP_AOE_Blast_FireStrike.BP_AOE_Blast_FireStrike_C" (Math|Transform|MakeTransform (Transformation|GetActorLocation AttackTarget) "0, 0, 0" "1.000000,1.000000,1.000000") "Undefined" "MultiplyWithRoot" 0 1.0 AttackTarget false false (Variables|Default|GetDraw%20Debug%20Type) 0))
          (EventDispatchers|AssignOnAoeOverlapActor _returnvalue (delegate Custom|OnAoeOverlapActor_Event)))))))

(event Custom|OnAoeOverlapActor_Event
  (params (Actor :type Actor%20Object%20Reference) (Hit%20Result :type Hit%20Result%20Structure))
  (bind (_damageinfo _damageamount _weapontype) (CallFunction|GetMainWeaponInfo))
  ;[1 1 1] Attack
  ;;[1 1 1] AOE Trail
  (bind _teamnumber (Class|BIDamagable|GetTeamNumber(Message) Actor))
  (if (!= _teamnumber (Variables|Default|GetTeamNumber))
    (Class|BIDamagable|TakeDamage(Message) Actor (Utilities|Struct|MakeS_DamageInfo _damageamount _weapontype) self Hit%20Result)))

(event Custom|AttackCombo1
  (params (AttackTarget :type Actor%20Object%20Reference))
  ;[1 1 1] Attack
  ;;[1 1 1] AttackCombo1
  (Default|BossPrimaryMeleeAttack (Variables|Default|GetAC_AttackComponent) (Utilities|Struct|MakeS_AttackInfo AttackTarget (Variables|Init|Montage|GetAttackCombo1_Montage) (.DamageInfo (CallFunction|GetMainWeaponInfo)))))

(event Custom|AttackCombo2
  (params (AttackTarget :type Actor%20Object%20Reference))
  (bind (_damageinfo _damageamount _weapontype) (CallFunction|GetMainWeaponInfo))
  ;[1 1 1] Attack
  ;;[1 1 1] AttackCombo2
  (CallFunction|Attack AttackTarget)
  (bind _notifyname (Animation|Montage|PlayMontage (Variables|Character|GetMesh) (Variables|Init|Montage|GetAttackCombo2_Montage))
    (:OnCompleted
      (CallFunction|AttackEnd AttackTarget :!label _label))
    (:OnInterrupted
      (goto _label))
    (:OnNotifyBegin
      (switch name _notifyname
        (:AoeSlash
          (Default|AOEDamage (Variables|Default|GetAC_AttackComponent) 2.5e+02 (Utilities|Struct|MakeS_DamageInfo _damageamount _weapontype) "200.000000,0.000000,0.000000"))))))

(event Custom|ThrowAxe
  (params (AttackTarget :type Actor%20Object%20Reference))
  (bind _equipedweapons (Variables|Default|GetEquipedWeapons))
  (bind _equipedweapons_2 (Variables|Default|GetEquipedWeapons))
  (bind _output (Utilities|Array|Get(acopy) _equipedweapons))
  (bind _output_2 (Utilities|Array|Get(acopy) _equipedweapons_2))
  ;[1 1 1] Attack
  ;;[1 1 1] ThrowAxe
  (CallFunction|Attack AttackTarget)
  (bind _notifyname (Animation|Montage|PlayMontage (Variables|Character|GetMesh) (Variables|Init|Montage|GetThrowAxe_Montage))
    (:OnCompleted
      (Utilities|IsValid _output :!label _label
        (:Is%20Valid
          (Rendering|SetVisibility (Variables|/Game/SoulsLikeBaseSystem/ComponentsAndSystem/WeaponSystem/BP_Weapon_Base.BP_Weapon_Base_C|GetMesh _output) true false))
        (:Is%20Not%20Valid
          _))
      (CallFunction|AttackEnd AttackTarget))
    (:OnInterrupted
      (goto _label))
    (:OnNotifyBegin
      (switch name _notifyname
        (:Throw
          (Utilities|IsValid _output_2
            (:Is%20Valid
              (Rendering|SetVisibility (Variables|/Game/SoulsLikeBaseSystem/ComponentsAndSystem/WeaponSystem/BP_Weapon_Base.BP_Weapon_Base_C|GetMesh _output_2) false false))
            (:Is%20Not%20Valid
              _))
          (bind _returnvalue (Game|SpawnActorfromClass "/Game/SoulsLikeBaseSystem/ComponentsAndSystem/ProjectilesSystem/BP_ThrowAxe.BP_ThrowAxe_C" (Math|Transform|MakeTransform (Transformation|GetSocketLocation (Variables|Character|GetMesh) (Variables|Default|GetMainWeaponSocketName)) "0, 0, 0" "1.000000,1.000000,1.000000") "Undefined" "MultiplyWithRoot" 0 4e+03 0.0 AttackTarget true self))
          (EventDispatchers|AssignOnProjectileImpact _returnvalue (delegate Custom|OnProjectileImpact_Event))
          (Collision|IgnoreActorwhenMoving (Variables|Default|GetCapsuleComponent) _returnvalue true))))))

(event Custom|OnProjectileImpact_Event
  (params (OtherActor :type Actor%20Object%20Reference) (Hit :type Hit%20Result%20Structure))
  (bind (_damageinfo _damageamount _weapontype) (CallFunction|GetMainWeaponInfo))
  ;[1 1 1] Attack
  ;;[1 1 1] ThrowAxe
  (bind _candamage (Default|CheckTeam (Variables|Default|GetAC_AttackComponent) OtherActor))
  (if _candamage
    (Class|BIDamagable|TakeDamage(Message) OtherActor (Utilities|Struct|MakeS_DamageInfo _damageamount _weapontype false true) self Hit)))

(event Custom|JumpAttack
  (params (AttackTarget :type Actor%20Object%20Reference))
  (bind (_damageinfo _damageamount _weapontype) (CallFunction|GetMainWeaponInfo))
  ;[1 1 1] Attack
  ;;[1 1 1] JumpAttack
  (Default|LongRangeMeleeAttack (Variables|Default|GetAC_AttackComponent) (Utilities|Struct|MakeS_AttackInfo AttackTarget (Variables|Init|Montage|GetJumpAttack_Montage) (Utilities|Struct|MakeS_DamageInfo _damageamount _weapontype false true)) "0, 0, 0"))

(event Custom|QuickAttack
  (params (AttackTarget :type Actor%20Object%20Reference))
  ;[1 1 1] Attack
  ;;[1 1 1] QuickAttack
  (Default|BossPrimaryMeleeAttack (Variables|Default|GetAC_AttackComponent) (Utilities|Struct|MakeS_AttackInfo AttackTarget (Variables|Init|Montage|GetQuickAttack_Montage) (.DamageInfo (CallFunction|GetMainWeaponInfo)))))

(event Custom|GroundSmash
  (params (AttackTarget :type Actor%20Object%20Reference))
  (bind (_damageinfo _damageamount _weapontype) (CallFunction|GetMainWeaponInfo))
  ;[1 1 1] Attack
  ;;[1 1 1] GroundSmash
  (Default|GroundSmashAOE (Variables|Default|GetAC_AttackComponent) (Utilities|Struct|MakeS_AttackInfo AttackTarget (Variables|Init|Montage|GetGroundSmash_Montage) (Utilities|Struct|MakeS_DamageInfo _damageamount _weapontype)) 1.1e+03 "0, 0, 0"))

(event EventBeginPlay
  (|CallParentFunction)
  (UserInterface|SetWidget (Variables|Default|GetHealthBar) 0)
  (bind _returnvalue (UserInterface|CreateWidget "/Game/SoulsLikeBaseSystem/HUD/WBP_BossHealthBar.WBP_BossHealthBar_C"))
  (Variables|Default|SetBossHealthBarWidgetRef _returnvalue)
  ;[1 1 1] Health bar
  (CallFunction|UpdateHealthBarEvent))

(event EventUpdateHealthBarEvent
  (bind _ac_statscomponent (Variables|Default|GetAC_StatsComponent))
  ;[1 1 1] Health bar Event Override
  (bind _bosshealthbarwidgetref (Variables|Default|GetBossHealthBarWidgetRef)
    (:then
      (Default|UpdateBossHelthBar _bosshealthbarwidgetref (Default|GetCurrentStats _ac_statscomponent "NewEnumerator1") (Default|GetMaxStats _ac_statscomponent "NewEnumerator1")))
    (:else)))

(event EventEquipWeaponBPI
  ;[1 1 1] Equip/ UnEquip
  (CallFunction|EquipMainWeaponsFunc (Variables|Default|GetEnemyMainWeapon) (Variables|Default|GetMainWeaponSocketName))
  (Utilities|FlowControl|DelayUntilNextTick)
  (Default|CallOnWeaponEquiped))

(event EventUnequipWeaponBPI
  ;[1 1 1] Equip/ UnEquip
  (CallFunction|UnEquipWeaponsFunc)
  (Utilities|FlowControl|DelayUntilNextTick)
  (Default|CallOnWeaponUnequiped))

(fn ConstructionScript
  (|CallParentFunction))

(fn TakeDamage
  (params (DamageInfo :type S%20Damage%20Info%20Structure) (Damage%20Causer :type Actor%20Object%20Reference) (Hit%20Result :type Hit%20Result%20Structure))
  (bind _ac_statscomponent (Variables|Default|GetAC_StatsComponent))
  (bind _wasdamaged (|CallParentFunction DamageInfo Damage%20Causer Hit%20Result))
  (Default|UpdateBossHelthBar (Variables|Default|GetBossHealthBarWidgetRef) (Default|GetCurrentStats _ac_statscomponent "NewEnumerator1") (Default|GetMaxStats _ac_statscomponent "NewEnumerator1"))
  (return _wasdamaged))