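; Base melee enemy Blueprint for a souls-like game that adds weapon equip and unequip handling and a set of melee attacks.
; Equip and unequip montages attach or remove the main weapon on notifies and signal completion when finished.
; Short-range, combo, long-range jump, spinning and AOE ground smash events pass montage, target and weapon damage to ACAttackComponent.
; Ground smash forces interrupts, while the spin attack is blockable.
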(event Custom|MeleeComboAttack
  (params (AttacoTarget :type Actor%20Object%20Reference))
  ;[1 1 1] Attack
  (Default|PrimaryMeleeAttack (Variables|Default|GetAC_AttackComponent) (Utilities|Struct|MakeS_AttackInfo AttacoTarget (Variables|Init|Montage|GetMelee_ComboAttack01) (.DamageInfo (CallFunction|GetMainWeaponInfo)))))

(event Custom|SpiningAttack
  (params (ActorTarget :type Actor%20Object%20Reference))
  (bind (_damageinfo _damageamount _weapontype) (CallFunction|GetMainWeaponInfo))
  ;[1 1 1] Attack
  (Default|SpiningMeleeAttack (Variables|Default|GetAC_AttackComponent) (Utilities|Struct|MakeS_AttackInfo ActorTarget (Variables|Init|Montage|GetMelee_SpinningAttack01) (Utilities|Struct|MakeS_DamageInfo _damageamount _weapontype false true))))

(event Custom|ShortRangeAttack
  (params (AttackTarget :type Actor%20Object%20Reference))
  ;[1 1 1] Attack
  (Default|PrimaryMeleeAttack (Variables|Default|GetAC_AttackComponent) (Utilities|Struct|MakeS_AttackInfo AttackTarget (Variables|Init|Montage|GetMelee_Attack01) (.DamageInfo (CallFunction|GetMainWeaponInfo)))))

(event Custom|LongRangeAttack
  (params (AttackTarget :type Actor%20Object%20Reference))
  ;[1 1 1] Attack
  (Default|LongRangeMeleeAttack (Variables|Default|GetAC_AttackComponent) (Utilities|Struct|MakeS_AttackInfo AttackTarget (Variables|Init|Montage|GetMelee_JumpAttack01) (.DamageInfo (CallFunction|GetMainWeaponInfo))) "0, 0, 0"))

(event Custom|GroundSmashAttack
  (params (AttackTarget :type Actor%20Object%20Reference))
  (bind (_damageinfo _damageamount _weapontype) (CallFunction|GetMainWeaponInfo))
  ;[1 1 1] Attack
  (Default|GroundSmashAOE (Variables|Default|GetAC_AttackComponent) (Utilities|Struct|MakeS_AttackInfo AttackTarget (Variables|Init|Montage|GetMelee_GroundSmash) (Utilities|Struct|MakeS_DamageInfo _damageamount _weapontype false false false true)) 3e+02 "200.000000,0.000000,0.000000"))

(event EventBeginPlay
  (|CallParentFunction))

(event EventUnequipWeaponBPI
  ;[1 1 1] Unequip weapon
  (bind _notifyname (Animation|Montage|PlayMontage (Variables|Character|GetMesh) (Variables|Init|Montage|GetUnequipWeapon_Montage))
    (:OnCompleted
      (Default|CallOnWeaponUnequiped))
    (:OnNotifyBegin
      (switch name _notifyname
        (:DropSword
          (CallFunction|UnEquipWeaponsFunc))))))

(event EventEquipWeaponBPI
  ;[1 1 1] Equip weapon
  (bind _notifyname (Animation|Montage|PlayMontage (Variables|Character|GetMesh) (Variables|Init|Montage|GetEquipWeapon_Montage))
    (:OnCompleted
      (Default|CallOnWeaponEquiped))
    (:OnNotifyBegin
      (switch name _notifyname
        (:HoldSword
          (CallFunction|EquipMainWeaponsFunc (Variables|Default|GetEnemyMainWeapon) (Variables|Default|GetMainWeaponSocketName)))))))

(fn ConstructionScript
  (|CallParentFunction))