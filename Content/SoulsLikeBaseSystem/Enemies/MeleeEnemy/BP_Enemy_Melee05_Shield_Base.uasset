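; Base Blueprint for a Souls-like melee enemy that, going by its name, carries a shield, handling drawing and stowing of its weapons.
; Blueprint interface events play equip or unequip montages on the mesh.
; Montage notifies time the attachment of main and secondary weapons to their sockets, or their removal.
; Montage completion calls the equipped or unequipped dispatcher, while other behavior comes from the parent class.
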(event EventBeginPlay
  (|CallParentFunction) ; This node is disabled and will not be called.\nDrag off pins to build functionality.
)

(event EventUnequipWeaponBPI
  ;[1 1 1] Unequip Weapon
  (bind _notifyname (Animation|Montage|PlayMontage (Variables|Character|GetMesh) (Variables|Default|GetUnequipWeapon_Montage))
    (:OnCompleted
      (Default|CallOnWeaponUnequiped))
    (:OnNotifyBegin
      (switch name _notifyname
        (:DropSword
          (CallFunction|UnEquipWeaponsFunc))))))

(event EventEquipWeaponBPI
  ;[1 1 1] Equip Weapon
  (bind _notifyname (Animation|Montage|PlayMontage (Variables|Character|GetMesh) (Variables|Default|GetEquipWeapon_Montage))
    (:OnCompleted
      (Default|CallOnWeaponEquiped))
    (:OnNotifyBegin
      (switch name _notifyname
        (:HoldSword
          (CallFunction|EquipMainWeaponsFunc (Variables|Default|GetEnemyMainWeapon) (Variables|Default|GetMainWeaponSocketName))
          (CallFunction|EquipMainWeaponsFunc (Variables|Default|GetEnemySecondaryWeapon) (Variables|Default|GetSecondaryWeaponSocketName)))))))

(event EventTick
  (params (DeltaSeconds :type Float%20%28single-precision%29)))

(event Collision|EventActorBeginOverlap
  (params (OtherActor :type Actor%20Object%20Reference)))

(fn ConstructionScript
  (|CallParentFunction))