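; Base projectile Blueprint for the Souls-like system's projectiles, with configurable speed, gravity, optional homing, and spawn and impact feedback.
; Construction applies the movement settings and, if homing, tracks the Target's root component.
; On BeginPlay it ignores its instigator (or owner) for collision, plays a spawn sound and aims its velocity at any Target.
; A box collision hit calls CallOnProjectileImpact, spawns impact effect and sound, then destroys the actor.
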(event OnComponentHit(BoxCollision)
  (params (HitComponent :type Primitive%20Component%20Object%20Reference) (OtherActor :type Actor%20Object%20Reference) (OtherComp :type Primitive%20Component%20Object%20Reference) (NormalImpulse :type Vector :default "0, 0, 0") (Hit :type Hit%20Result%20Structure%20%28by%20ref%29))
  (bind _location (Collision|BreakHitResult Hit))
  ;[1 1 1] Hit Something
  (Default|CallOnProjectileImpact OtherActor Hit)
  (Niagara|SpawnSystematLocation (Variables|Init|GetImpactEffect) _location)
  (Audio|PlaySoundatLocation (Variables|Init|GetImpactSound) _location "0, 0, 0" 1.0 1.0 0.0 0 0 0 0)
  (Actor|DestroyActor))

(event Custom|RotateToTarget
  ;[1 1 1] Rotate To Target
  (Variables|/Script/Engine.MovementComponent|SetVelocity (Variables|Default|GetProjectileMovement) (* (Math|Vector|GetUnitDirection(Vector) (Transformation|GetActorLocation) (Transformation|GetActorLocation (Variables|Default|GetTarget))) (Variables|Init|GetSpeed))))

(event Custom|PlaySpawnSound
  ;[1 1 1] Player Spawn Sound
  (Audio|PlaySoundatLocation (Variables|Init|GetSpawnSound) (Transformation|GetActorLocation) "0, 0, 0" 1.0 1.0 0.0 0 0 0 0))

(event EventBeginPlay
  (bind _returnvalue (Game|GetInstigator))
  ;[1 1 1] Ignore Self
  (Collision|IgnoreActorwhenMoving (Variables|Default|GetBoxCollision) (select (Utilities|IsValid _returnvalue) _returnvalue (Components|GetOwner)) true)
  ;[1 1 1] Play Spwn Sound
  (CallFunction|PlaySpawnSound)
  ;[1 1 1] Rotate To target
  (Variables|Default|GetTarget
    (:then
      (CallFunction|RotatetoTarget))
    (:else)))

(fn ConstructionScript
  (bind _projectilemovement (Variables|Default|GetProjectileMovement))
  (bind _projectilemovement_2 (Variables|Default|GetProjectileMovement))
  (Variables|/Script/Engine.ProjectileMovementComponent|SetInitialSpeed _projectilemovement (Variables|Init|GetSpeed))
  (Variables|/Script/Engine.ProjectileMovementComponent|SetMaxSpeed _projectilemovement (Variables|Init|GetSpeed))
  (Variables|/Script/Engine.ProjectileMovementComponent|SetProjectileGravityScale _projectilemovement (Variables|Init|GetGravity))
  (Variables|Default|GetTarget
    (:then
      (if (Variables|Init|GetIsHoming)
        (Variables|/Script/Engine.ProjectileMovementComponent|SetbIsHomingProjectile _projectilemovement_2 true)
        (Variables|/Script/Engine.ProjectileMovementComponent|SetHomingTargetComponent _projectilemovement_2 (Variables|/Script/Engine.Actor|GetRootComponent (Variables|Default|GetTarget)))))
    (:else)))