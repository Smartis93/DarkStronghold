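; Base Blueprint for blast-type area-of-effect actors in the Souls-like AOE system, extending the parent's Trigger event with visual and audio feedback.
; On Trigger it runs the parent logic, spawns the blast effect attached to its root, and plays the sound at its location.
; The actor destroys itself when the effect system finishes, or after a short delay when no effect is set.
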(event Custom|OnSystemFinished_Event
  (params (PSystem :type Niagara%20Component%20Object%20Reference))
  (Actor|DestroyActor))

(event Custom|SpawnBlastEffect
  (bind _blasteffect (Variables|Init|GetBlastEffect)
    (:then
      (bind _returnvalue (Niagara|SpawnSystemAttached _blasteffect (Variables|Default|GetDefaultSceneRoot) "None" "0, 0, 0" "0, 0, 0" "KeepRelativeOffset" false))
      (EventDispatchers|AssignOnSystemFinished _returnvalue (delegate Custom|OnSystemFinished_Event)))
    (:else
      (Utilities|FlowControl|Delay 1.0)
      (Actor|DestroyActor))))

(event Custom|PlayBlastSound
  (bind _sound (Variables|Init|GetSound)
    (:then
      (Audio|PlaySoundatLocation _sound (Transformation|GetActorLocation) "0, 0, 0" 1.0 1.0 0.0 0 0 0 0))
    (:else)))

(event EventBeginPlay
  (|CallParentFunction) ; This node is disabled and will not be called.\nDrag off pins to build functionality.
)

(event Collision|EventActorBeginOverlap
  (params (OtherActor :type Actor%20Object%20Reference)))

(event EventTick
  (params (DeltaSeconds :type Float%20%28single-precision%29)))

(event EventTrigger
  (|CallParentFunction)
  (CallFunction|SpawnBlastEffect)
  (CallFunction|PlayBlastSound))

(fn ConstructionScript
  (|CallParentFunction))