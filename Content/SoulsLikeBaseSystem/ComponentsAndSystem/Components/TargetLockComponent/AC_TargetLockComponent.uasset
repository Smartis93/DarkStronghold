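; Souls-like target lock component for a Character that keeps the camera and character facing a chosen enemy.
; Camera-forward sphere traces find living BI_EnemyAI actors, and toggling switches to a random other hit.
; Tick interpolates control rotation toward the target and releases it beyond the lost-lock distance.
; Locking switches movement between camera and movement orientation, notifies the target, and relays its AC_DamageSystem death through a dispatcher.
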(event Custom|EnableLockOn
  ;[1 1 1] Enable Lock On
  (bind (_value _targetactor) (CallFunction|FindTarget))
  (if _value
    (bind _output_get (Variables|Default|SetLockOnTargetActor _targetactor))
    (EventDispatchers|AssignOnDeath (Actor|GetComponentbyClass _output_get "/Game/SoulsLikeBaseSystem/ComponentsAndSystem/Components/DamageComponent/AC_DamageSystem.AC_DamageSystem_C") (delegate Custom|OnDeath_Event))
    (CallFunction|SetIsTargeting true)
    (CallFunction|SetMoveMode "NewEnumerator0")))

(event Custom|DisableLockOn
  ;[1 1 1] Disable Lock On
  (CallFunction|SetIsTargeting false)
  (Variables|Default|SetLockOnTargetActor 0)
  (CallFunction|SetMoveMode "NewEnumerator1"))

(event Custom|StartLockOnTarget
  ;[1 1 1] StartLockOnTarget
  (if (not (Variables|Default|GetIsTargeting))
    (CallFunction|EnableLockon)
    (else
      (CallFunction|DisableLockon))))

(event Custom|TargetDeath
  ;[1 1 1] Toggle Target
  (Default|CallOnLockonTargetActorDeath))

(event Custom|ToggleTarget
  ;[1 1 1] Toggle Target
  (bind (_value _targetactor) (CallFunction|ToggleTargetFunc))
  (if _value
    (bind _output_get (Variables|Default|SetLockOnTargetActor _targetactor))
    (Utilities|IsValid (Actor|GetComponentbyClass _output_get "/Game/SoulsLikeBaseSystem/ComponentsAndSystem/Components/DamageComponent/AC_DamageSystem.AC_DamageSystem_C")
      (:Is%20Valid
        (EventDispatchers|AssignOnDeath (Actor|GetComponentbyClass _output_get "/Game/SoulsLikeBaseSystem/ComponentsAndSystem/Components/DamageComponent/AC_DamageSystem.AC_DamageSystem_C") (delegate Custom|TargetDeath))
        (CallFunction|SetIsTargeting true)
        (CallFunction|SetMoveMode "NewEnumerator0")))))

(event Custom|OnDeath_Event
  ;[1 1 1] Enable Lock On
  (Default|CallOnLockonTargetActorDeath))

(event EventBeginPlay
  (bind _ascharacter (Utilities|Casting|CastToCharacter (Components|GetOwner)))
  (Variables|Default|SetOwnerCharacterRef _ascharacter)
  (Variables|Default|SetOwnerControllerRef (Pawn|GetController (Variables|Default|GetOwnerCharacterRef)))
  (Utilities|IsValid (Actor|GetComponentbyClass (Variables|Default|GetOwnerCharacterRef) "/Script/Engine.CameraComponent")
    (:Is%20Valid
      (Variables|Default|SetOwnerFollowCameraRef (Actor|GetComponentbyClass (Variables|Default|GetOwnerCharacterRef) "/Script/Engine.CameraComponent")))))

(event EventTick
  (params (DeltaSeconds :type Float%20%28single-precision%29))
  ;[1 1 1] Tick  Rotate to target
  (bind _lockontargetactor (Variables|Default|GetLockOnTargetActor)
    (:then
      (if (CallFunction|CanLockingTargetActor _lockontargetactor)
        (CallFunction|UpdateTargetingRotation)
        (else
          (CallFunction|DisableLockon))))
    (:else)))

(fn FindTarget
  (bind _returnvalue (Components|GetOwner))
  (bind _returnvalue_2 (Transformation|GetActorLocation _returnvalue))
  (bind (_outhit _returnvalue_3) (Collision|SphereTraceForObjects _returnvalue_2 (+ _returnvalue_2 (* (Math|Vector|GetForwardVector (Variables|Default|GetOwnerFollowCameraRef)) (Variables|Init|GetLockTargetRange))) (Variables|Init|GetLockTargetRadius) (Variables|Init|GetTargetObjectTypes) false (Utilities|Array|MakeArray (Components|GetOwner)) (Variables|Init|GetDraw%20Debug%20Type)))
  (if (and _returnvalue_3 (Utilities|DoesObjectImplementInterface (.HitActor (Collision|BreakHitResult _outhit)) "/Game/SoulsLikeBaseSystem/Enemies/AI/Interface/BI_EnemyAI.BI_EnemyAI_C"))
    (bind _isdead (Class|BIDamagable|IsDead(Message) (.HitActor (Collision|BreakHitResult _outhit))))
    (if _isdead
      _
      (else
        (return true (.HitActor (Collision|BreakHitResult _outhit))))))
  (return false 0))

(fn UpdateTargetingRotation
  (bind _returnvalue (Utilities|Time|GetWorldDeltaSeconds))
  (bind _returnvalue_2 (Components|GetOwner))
  (bind _ownercontrollerref (Variables|Default|GetOwnerControllerRef))
  (bind _lockontargetactor (Variables|Default|GetLockOnTargetActor))
  (bind _rotatetotargetinterpspeed (Variables|Init|GetRotateToTargetInterpSpeed))
  (bind _returnvalue_3 (Transformation|GetActorLocation _lockontargetactor))
  (bind _returnvalue_4 (Transformation|GetActorRotation _ownercontrollerref))
  (bind _returnvalue_5 (Transformation|GetActorLocation _returnvalue_2))
  (bind _returnvalue_6 (- _returnvalue_3 "0.000000,0.000000,100.000000"))
  (bind _returnvalue_7 (Math|Rotator|FindLookatRotation _returnvalue_5 _returnvalue_6))
  (bind _returnvalue_8 (Math|Interpolation|RInterpTo _returnvalue_4 _returnvalue_7 _returnvalue _rotatetotargetinterpspeed))
  (if (and (Utilities|IsValid (Variables|Default|GetOwnerControllerRef)) (Utilities|IsValid (Variables|Default|GetLockOnTargetActor)))
    (Pawn|SetControlRotation (Variables|Default|GetOwnerControllerRef) (Math|Rotator|MakeRotator (.Roll (Math|Rotator|BreakRotator _returnvalue_4)) (.pitch _returnvalue_8) (.yaw _returnvalue_8)))))

(fn SetMoveMode
  (params (NewMoveMode :type E_MoveMode%20Enum :default "NewEnumerator0"))
  (bind _ownercharacterref (Variables|Default|GetOwnerCharacterRef))
  (bind _charactermovement (Variables|/Script/Engine.Character|GetCharacterMovement _ownercharacterref))
  (bind _output_get (Variables|Default|SetMoveMode NewMoveMode))
  (switch Utilities|FlowControl|Switch|SwitchonE_MoveMode _output_get
    (:NewEnumerator0
      (Variables|/Script/Engine.CharacterMovementComponent|SetbOrientRotationToMovement _charactermovement false)
      (Variables|/Script/Engine.CharacterMovementComponent|SetbUseControllerDesiredRotation _charactermovement true)
      (Variables|/Script/Engine.CharacterMovementComponent|SetbUseControllerDesiredRotation _charactermovement true))
    (:NewEnumerator1
      (Variables|/Script/Engine.CharacterMovementComponent|SetbOrientRotationToMovement _charactermovement true)
      (Variables|/Script/Engine.CharacterMovementComponent|SetbUseControllerDesiredRotation _charactermovement false)
      (Variables|/Script/Engine.CharacterMovementComponent|SetbUseControllerDesiredRotation _charactermovement false))))

(fn CheckDistancetoTargetActorinRange
  (params (LockOnTargetActor :type Actor%20Object%20Reference))
  (return (< (Transformation|GetDistanceTo LockOnTargetActor (Components|GetOwner)) (Variables|Default|GetLostLockTargetDistance))))

(fn CanLockingTargetActor
  (params (LockOnTargetActor :type Actor%20Object%20Reference))
  (return (and (Variables|Default|GetIsTargeting) (CallFunction|CheckDistancetoTargetActorinRange LockOnTargetActor))))

(fn SetIsTargeting
  (params (IsTargeting :type Boolean))
  (bind _output_get (Variables|Default|SetIsTargeting IsTargeting))
  (bind _lockontargetactor (Variables|Default|GetLockOnTargetActor)
    (:then
      (Class|BITarget|OnLockonTarget(Message) _lockontargetactor _output_get))
    (:else)))

(fn ToggleTargetFunc
  (bind _returnvalue (Components|GetOwner))
  (bind _l_lockontargetactor (LocalVariables|GetL_LockOnTargetActor))
  (bind _returnvalue_2 (Transformation|GetActorLocation _returnvalue))
  (bind (_outhits _returnvalue_3) (Collision|MultiSphereTraceForObjects _returnvalue_2 (+ _returnvalue_2 (* (Math|Vector|GetForwardVector (Variables|Default|GetOwnerFollowCameraRef)) (Variables|Init|GetLockTargetRange))) (Variables|Init|GetLockTargetRadius) (Variables|Init|GetTargetObjectTypes) false (Utilities|Array|MakeArray (Components|GetOwner)) (Variables|Init|GetDraw%20Debug%20Type)))
  (if _returnvalue_3
    (for _array_element _outhits
      (if (Utilities|DoesObjectImplementInterface (.HitActor (Collision|BreakHitResult _array_element)) "/Game/SoulsLikeBaseSystem/Enemies/AI/Interface/BI_EnemyAI.BI_EnemyAI_C")
        (bind _isdead (Class|BIDamagable|IsDead(Message) (.HitActor (Collision|BreakHitResult _array_element))))
        (if _isdead
          (return false 0)
          (else
            (Utilities|Array|AddUnique (LocalVariables|GetL_LockOnTargetActor) (.HitActor (Collision|BreakHitResult _array_element)))))
        (else
          (return false 0))))
    (bind _lockontargetactor (Variables|Default|GetLockOnTargetActor)
      (:then
        (if (> (Utilities|Array|Length (LocalVariables|GetL_LockOnTargetActor)) 1)
          (Class|BITarget|OnLockonTarget(Message) _lockontargetactor false)
          (Utilities|Array|RemoveItem _l_lockontargetactor _lockontargetactor)
          (bind _output_get (Variables|Default|SetLockOnTargetActor (.OutItem (Utilities|Array|Random _l_lockontargetactor))))
          (return true _output_get)))
      (:else))
    (else
      (return false 0))))