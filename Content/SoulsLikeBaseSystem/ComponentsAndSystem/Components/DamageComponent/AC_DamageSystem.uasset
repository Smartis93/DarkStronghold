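; Actor component that resolves incoming hits, healing and attack tokens for its owner in a souls-like combat system.
; TakeDamage filters on death, invincibility and frontal blocking, using a dot/cross angle to classify hit direction.
; Hits subtract summed damage from health and adjust weapon-specific stability through AC_StatsComponent.
; It then calls handlers for block, damage FX, death, stability depletion or interrupt response.
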(event EventBeginPlay
  (bind _returnvalue (Components|GetOwner))
  (bind _returnvalue_2 (Actor|GetComponentbyClass _returnvalue "/Game/SoulsLikeBaseSystem/ComponentsAndSystem/Components/BaseStatsComponent/AC_StatsComponent.AC_StatsComponent_C"))
  (Utilities|IsValid _returnvalue_2
    (:Is%20Valid
      (Variables|Default|SetStatsComponent _returnvalue_2))))

(fn Heal
  (params (Amount :type Float%20%28double-precision%29))
  (if (not (Variables|Default|GetIsDead))
    (bind _newvalue (Default|ModifyCurrentStats (Variables|Default|GetStatsComponent) "NewEnumerator1" Amount))
    (return _newvalue)))

(fn TakeDamage
  (params (DamageInfo :type S%20Damage%20Info%20Structure) (DamageCauser :type Actor%20Object%20Reference) (HitResult :type Hit%20Result%20Structure))
  (bind (_damageamount _weapontype _shoulddamageinvincible _canbeblocked _canbeparried _shouldforceinterrupt) (Utilities|Struct|BreakS_DamageInfo DamageInfo))
  (Utilities|CanbeDamaged _shoulddamageinvincible _canbeblocked DamageCauser
    (:BlockDamage
      (Default|CallOnBlocked _canbeparried DamageCauser)
      (return false))
    (:DoDamage
      (CallFunction|CalculateCurrentHealth _damageamount)
      (Default|CallOnDamageFX _damageamount HitResult)
      (if (Variables|Default|GetIsDead)
        (Default|CallOnDeath)
        (else
          (bind _stablevalueiszero (CallFunction|CalculateStableValue _weapontype))
          (if _stablevalueiszero
            (if (Variables|Default|GetIsStun)
              _
              (else
                (Default|CallOnStableValueZero DamageCauser)))
            (elif (or (Variables|Default|GetCanBeInterruptible) _shouldforceinterrupt)
              (Default|CallOnDamageResponse DamageCauser _weapontype)))))
      (return true))
    (:NoDamage
      (return false))))

(fn ReserveAttackToken
  (params (Amount :type Integer))
  (if (>= (Variables|Init|GetAttackTokensCount) Amount)
    (Variables|Init|SetAttackTokensCount (- (Variables|Init|GetAttackTokensCount) Amount))
    (return true)
    (else
      (return false))))

(fn ReturnAttackToken
  (params (Amount :type Integer))
  (Variables|Init|SetAttackTokensCount (+ Amount (Variables|Init|GetAttackTokensCount)))
  (return))

(fn CalculateDamage
  (params (DamageAmount :type Map%20of%20E_DamageType%20Enums%20to%20Reals :default "NewEnumerator0"))
  (return (+ (.Value (Utilities|Map|Find DamageAmount "NewEnumerator0")) (.Value (Utilities|Map|Find DamageAmount "NewEnumerator1")) (.Value (Utilities|Map|Find DamageAmount "NewEnumerator2")) (.Value (Utilities|Map|Find DamageAmount "NewEnumerator3")) (.Value (Utilities|Map|Find DamageAmount "NewEnumerator4")))))

(fn CalculateCurrentHealth
  (params (DamageAmount :type Map%20of%20E_DamageType%20Enums%20to%20Reals :default "NewEnumerator0"))
  (Default|ModifyCurrentStats (Variables|Default|GetStatsComponent) "NewEnumerator1" (* (CallFunction|CalculateDamage DamageAmount) -1.0))
  (return))

(fn CalculateStableValue
  (params (WeaponType :type E_WeaponType%20Enum :default "NewEnumerator0"))
  (bind _statscomponent (Variables|Default|GetStatsComponent))
  (switch Utilities|FlowControl|Switch|SwitchonE_WeaponType WeaponType
    (:NewEnumerator0
      (Default|ModifyCurrentStats (Variables|Default|GetStatsComponent) "NewEnumerator3" 0.0))
    (:NewEnumerator1
      (Default|ModifyCurrentStats (Variables|Default|GetStatsComponent) "NewEnumerator3" (Variables|Init|GetSwordReduceStable)))
    (:NewEnumerator2
      (Default|ModifyCurrentStats (Variables|Default|GetStatsComponent) "NewEnumerator3" (Variables|Init|GetSingleHandAxeReduceStable)))
    (:NewEnumerator3
      (Default|ModifyCurrentStats (Variables|Default|GetStatsComponent) "NewEnumerator3" (Variables|Init|GetMagicHandReduceStable)))
    (:NewEnumerator4
      (Default|ModifyCurrentStats (Variables|Default|GetStatsComponent) "NewEnumerator3" (Variables|Init|GetRifleReduceStable)))
    (:NewEnumerator5
      (Default|ModifyCurrentStats (Variables|Default|GetStatsComponent) "NewEnumerator3" (Variables|Init|GetShieldReduceStable))))
  (if (< (Default|GetCurrentStats _statscomponent "NewEnumerator3") (Default|GetMaxStats _statscomponent "NewEnumerator3"))
    (Default|CallOnStableValueReduce)
    (return (<= (Default|GetCurrentStats (Variables|Default|GetStatsComponent) "NewEnumerator3") 0.0))
    (else
      (return false))))

(fn IntervalDamage
  (params (DamageHealthPercent :type Float%20%28double-precision%29) (CurrentHealth :type Float%20%28double-precision%29) (MaxHealth :type Float%20%28double-precision%29))
  (Default|SetCurrentStats (Variables|Default|GetStatsComponent) "NewEnumerator1" (- CurrentHealth (* DamageHealthPercent MaxHealth))))

(fn CalculateDirectionTheta
  (params (DamageCauser :type Actor%20Object%20Reference) (DamagedActor :type Actor%20Object%20Reference))
  (bind _returnvalue (Transformation|GetActorLocation DamagedActor))
  (bind _returnvalue_2 (Transformation|GetActorLocation DamageCauser))
  (bind _returnvalue_3 (Transformation|GetActorForwardVector DamagedActor))
  (bind _returnvalue_4 (- _returnvalue_2 _returnvalue))
  (bind _returnvalue_5 (Math|Vector|Normalize _returnvalue_4))
  (bind _returnvalue_6 (Math|Vector|DotProduct _returnvalue_3 _returnvalue_5))
  (bind _returnvalue_7 (Math|Trig|Acos(Degrees) _returnvalue_6))
  (if (< (.z (Math|Vector|CrossProduct _returnvalue_3 _returnvalue_5)) 0.0)
    (LocalVariables|SetL_Theta (Math|Trig|RadiansToDegrees (* _returnvalue_7 -1.0)))
    (else
      (LocalVariables|SetL_Theta (Math|Trig|RadiansToDegrees _returnvalue_7))))
  (return (LocalVariables|GetL_Theta)))