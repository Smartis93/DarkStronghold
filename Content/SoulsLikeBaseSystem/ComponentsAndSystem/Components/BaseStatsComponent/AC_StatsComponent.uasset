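; Souls-like actor component that holds a character's health, mana, stamina and stable stats plus attributes, all stored in maps.
; On BeginPlay it derives each max stat from base values and weighted attributes, then fills current stats to max.
; Modify functions clamp changes and fire dispatchers for stat zero, max and change, and attribute change or max.
; It also computes attribute-scaled damage, defense with armor, and final damage as Damage squared over Defense.
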(event EventBeginPlay
  ;[1 1 1] Initialize Stats
  (CallFunction|Initialize))

(fn SetCurrentStats
  (params (Stats :type E_Stats%20Enum :default "NewEnumerator0") (Value :type Float%20%28double-precision%29))
  (Utilities|Map|Add (Variables|Stats|GetCurrentStats) Stats Value)
  (return Value))

(fn GetCurrentStats
  (params (Stats :type E_Stats%20Enum :default "NewEnumerator0"))
  (return (.Value (Utilities|Map|Find (Variables|Stats|GetCurrentStats) Stats))))

(fn SetMaxStats
  (params (Stats :type E_Stats%20Enum :default "NewEnumerator0") (Value :type Float%20%28double-precision%29))
  (Utilities|Map|Add (Variables|Stats|GetMaxStats) Stats Value)
  (return Value))

(fn Initialize
  (bind _keys (Utilities|Map|Keys (Variables|Stats|GetCurrentStats)))
  (for _array_element _keys
    (bind _value (Stats|CalculationMaxStats _array_element))
    (Stats|SetCurrentStats _array_element _value)))

(fn GetMaxStats
  (params (Stats :type E_Stats%20Enum :default "NewEnumerator0"))
  (return (.Value (Utilities|Map|Find (Variables|Stats|GetMaxStats) Stats))))

(fn CalculationMaxStats
  (params (Stats :type E_Stats%20Enum :default "NewEnumerator0"))
  (bind _value (Attributes|GetCurrentAttributes "NewEnumerator5"))
  (bind _value_2 (Attributes|GetCurrentAttributes "NewEnumerator6"))
  (bind _value_3 (Attributes|GetCurrentAttributes "NewEnumerator4"))
  (bind _value_4 (Attributes|GetCurrentAttributes "NewEnumerator5"))
  (bind _value_5 (Attributes|GetCurrentAttributes "NewEnumerator6"))
  (bind _value_6 (Attributes|GetCurrentAttributes "NewEnumerator4"))
  (bind _manamultiple (Variables|Initial|GetManaMultiple))
  (bind _staminamultiple (Variables|Initial|GetStaminaMultiple))
  (bind _stablemultiple (Variables|Initial|GetStableMultiple))
  (bind _stablemultiple_2 (Variables|Initial|GetStableMultiple))
  (bind _stablemultiple_3 (Variables|Initial|GetStableMultiple))
  (bind _initialhealth (Variables|Initial|GetInitialHealth))
  (bind _initialmana (Variables|Initial|GetInitialMana))
  (bind _initialstamina (Variables|Initial|GetInitialStamina))
  (bind _initialstable (Variables|Initial|GetInitialStable))
  (bind _healthmultiple (Variables|Initial|GetHealthMultiple))
  (bind _returnvalue (* _value_6 _stablemultiple_3))
  (bind _returnvalue_2 (* _value _healthmultiple))
  (bind _returnvalue_3 (* _value_2 _manamultiple))
  (bind _returnvalue_4 (* _value_3 _staminamultiple))
  (bind _returnvalue_5 (* _value_4 _stablemultiple))
  (bind _returnvalue_6 (* _value_5 _stablemultiple_2))
  (bind _returnvalue_7 (+ _initialstable _returnvalue_5 _returnvalue_6 _returnvalue))
  (bind _returnvalue_8 (+ _initialhealth _returnvalue_2))
  (bind _returnvalue_9 (+ _initialmana _returnvalue_3))
  (bind _returnvalue_10 (+ _initialstamina _returnvalue_4))
  (bind _output_get (LocalVariables|SetStats_L Stats))
  (switch Utilities|FlowControl|Switch|SwitchonE_Stats _output_get
    (:NewEnumerator1
      ;[1 1 1] Init Max Health
      (Stats|SetMaxStats (LocalVariables|GetStats_L) _returnvalue_8)
      (return _returnvalue_8))
    (:NewEnumerator15
      ;[1 1 1] Init Max Mana
      (Stats|SetMaxStats (LocalVariables|GetStats_L) _returnvalue_9)
      (return _returnvalue_9))
    (:NewEnumerator2
      ;[1 1 1] Init Max Stamina
      (Stats|SetMaxStats (LocalVariables|GetStats_L) _returnvalue_10)
      (return _returnvalue_10))
    (:NewEnumerator3
      ;[1 1 1] Init Max Stable
      (Stats|SetMaxStats (LocalVariables|GetStats_L) _returnvalue_7)
      (return _returnvalue_7))))

(fn ModifyCurrentStats
  (params (Stat :type E_Stats%20Enum :default "NewEnumerator0") (Value :type Float%20%28double-precision%29))
  (if (!= Value 0.0)
    (LocalVariables|SetStat_L Stat)
    (LocalVariables|SetValue_L (Math|Float|Clamp(Float) (+ Value (Stats|GetCurrentStats (LocalVariables|GetStat_L))) 0.0 (Stats|GetMaxStats (LocalVariables|GetStat_L))))
    (switch Utilities|FlowControl|Switch|SwitchonE_Stats (LocalVariables|GetStat_L)
      (:NewEnumerator1
        ;[1 1 1] Health
        (if (<= (LocalVariables|GetValue_L) 0.0)
          (Default|CallOnCurrentHealthIsZero)
          (elif (>= (LocalVariables|GetValue_L) (Stats|GetMaxStats (LocalVariables|GetStat_L)))
            (Default|CallOnCurrentHealthReachesMax)))
        (Stats|SetCurrentStats (LocalVariables|GetStat_L) (LocalVariables|GetValue_L))
        (Default|CallOnCurrentHealthChanged)
        (return (LocalVariables|GetValue_L)))
      (:NewEnumerator15
        ;[1 1 1] Mana
        (if (<= (LocalVariables|GetValue_L) 0.0)
          (Default|CallOnCurrentManaIsZero)
          (elif (>= (LocalVariables|GetValue_L) (Stats|GetMaxStats (LocalVariables|GetStat_L)))
            (Default|CallOnCurrentManaReachesMax)))
        (Stats|SetCurrentStats (LocalVariables|GetStat_L) (LocalVariables|GetValue_L))
        (Default|CallOnCurrentManaChanged)
        (return (LocalVariables|GetValue_L)))
      (:NewEnumerator2
        ;[1 1 1] Stamina
        (if (<= (LocalVariables|GetValue_L) 0.0)
          (Default|CallOnCurrentStaminaIsZero)
          (elif (>= (LocalVariables|GetValue_L) (Stats|GetMaxStats (LocalVariables|GetStat_L)))
            (Default|CallOnCurrentStaminaReachesMax)))
        (Stats|SetCurrentStats (LocalVariables|GetStat_L) (LocalVariables|GetValue_L))
        (Default|CallOnCurrentStaminaChanged)
        (return (LocalVariables|GetValue_L)))
      (:NewEnumerator3
        ;[1 1 1] Stable
        (if (<= (LocalVariables|GetValue_L) 0.0)
          (Default|CallOnCurrentStableIsZero)
          (elif (>= (LocalVariables|GetValue_L) (Stats|GetMaxStats (LocalVariables|GetStat_L)))
            (Default|CallOnCurrentStableReachesMax)))
        (Stats|SetCurrentStats (LocalVariables|GetStat_L) (LocalVariables|GetValue_L))
        (Default|CallOnCurrentStableChanged)
        (return (LocalVariables|GetValue_L))))
    (else
      (Development|PrintString "Modify Current State Value Equal Zero"))))

(fn ModifyMaxStats
  (params (Stat :type E_Stats%20Enum :default "NewEnumerator0") (Value :type Float%20%28double-precision%29))
  (bind _value (Stats|GetMaxStats Stat))
  (bind _returnvalue (+ Value _value))
  (Stats|SetMaxStats Stat _returnvalue)
  (return _returnvalue))

(fn SetCurrentAttributes
  (params (Attribute :type E_Attributes%20Enum :default "NewEnumerator0") (Value :type Float%20%28double-precision%29))
  (Utilities|Map|Add (Variables|Attributes|GetCurrentAttributes) Attribute Value)
  (return Value))

(fn GetCurrentAttributes
  (params (Attributes :type E_Attributes%20Enum :default "NewEnumerator0"))
  (return (.Value (Utilities|Map|Find (Variables|Attributes|GetCurrentAttributes) Attributes))))

(fn GetMaxAttributes
  (params (Attributes :type E_Attributes%20Enum :default "NewEnumerator0"))
  (return (.Value (Utilities|Map|Find (Variables|Attributes|GetMaxAttributes) Attributes))))

(fn ModifyCurrentAttributes
  (params (Attribute :type E_Attributes%20Enum :default "NewEnumerator0") (Value :type Float%20%28double-precision%29))
  (if (!= Value 0.0)
    (LocalVariables|SetAttribute_L Attribute)
    (LocalVariables|SetValue_L (Math|Float|Clamp(Float) (+ Value (.Value (Utilities|Map|Find (Variables|Attributes|GetCurrentAttributes) (LocalVariables|GetAttribute_L)))) 0.0 (Attributes|GetMaxAttributes (LocalVariables|GetAttribute_L))))
    (if (>= (LocalVariables|GetValue_L) (Attributes|GetMaxAttributes (LocalVariables|GetAttribute_L)))
      (Default|CallOnAttributeReachesMax (LocalVariables|GetAttribute_L)))
    (Attributes|SetCurrentAttributes (LocalVariables|GetAttribute_L) (LocalVariables|GetValue_L))
    (Default|CallOnAttributeChanged (LocalVariables|GetAttribute_L))
    (return (LocalVariables|GetValue_L))))

(fn GetDamage
  (params (DamageType :type E_Damage%20Enum :default "NewEnumerator4") (WeaponDamage :type Float%20%28double-precision%29))
  (LocalVariables|SetWeaponDamage_L WeaponDamage)
  (switch Utilities|FlowControl|Switch|SwitchonE_Damage DamageType
    (:NewEnumerator0
      ;[1 1 1] MeleeDamage
      (return (+ (LocalVariables|GetWeaponDamage_L) (* (LocalVariables|GetWeaponDamage_L) (* (Attributes|GetCurrentAttributes "NewEnumerator1") (Variables|Initial|GetDamageMultiple))))))
    (:NewEnumerator6
      ;[1 1 1] RangeDamage
      (return (+ (LocalVariables|GetWeaponDamage_L) (* (LocalVariables|GetWeaponDamage_L) (* (Attributes|GetCurrentAttributes "NewEnumerator2") (Variables|Initial|GetDamageMultiple))))))
    (:NewEnumerator1
      ;[1 1 1] MagicDamage
      (return (+ (LocalVariables|GetWeaponDamage_L) (* (LocalVariables|GetWeaponDamage_L) (* (Attributes|GetCurrentAttributes "NewEnumerator3") (Variables|Initial|GetDamageMultiple))))))))

(fn GetDefense
  (params (DefenseStats :type E_Defense%20Enum :default "NewEnumerator4") (ArmorPhysicDefense :type Float%20%28double-precision%29) (ArmorMagicDefense :type Float%20%28double-precision%29))
  (bind _defensemultiple (Variables|Initial|GetDefenseMultiple))
  (bind _defensemultiple_2 (Variables|Initial|GetDefenseMultiple))
  (LocalVariables|SetArmorPhysicDefense_L ArmorPhysicDefense)
  (LocalVariables|SetArmorMagicDefense_L ArmorMagicDefense)
  (switch Utilities|FlowControl|Switch|SwitchonE_Defense DefenseStats
    (:NewEnumerator2
      ;[1 1 1] PhysicalDefensePercentage
      (return (+ (+ (* (Attributes|GetCurrentAttributes "NewEnumerator5") _defensemultiple) (* (Attributes|GetCurrentAttributes "NewEnumerator6") _defensemultiple) (* (Attributes|GetCurrentAttributes "NewEnumerator4") _defensemultiple) (* (Attributes|GetCurrentAttributes "NewEnumerator1") _defensemultiple) (* (Attributes|GetCurrentAttributes "NewEnumerator2") _defensemultiple) (* (Attributes|GetCurrentAttributes "NewEnumerator3") _defensemultiple)) (Variables|Initial|GetInitialDefense) (LocalVariables|GetArmorPhysicDefense_L))))
    (:NewEnumerator3
      ;[1 1 1] MagicDefensePercentage
      (return (+ (+ (* (Attributes|GetCurrentAttributes "NewEnumerator5") _defensemultiple_2) (* (Attributes|GetCurrentAttributes "NewEnumerator6") _defensemultiple_2) (* (Attributes|GetCurrentAttributes "NewEnumerator4") _defensemultiple_2) (* (Attributes|GetCurrentAttributes "NewEnumerator1") _defensemultiple_2) (* (Attributes|GetCurrentAttributes "NewEnumerator2") _defensemultiple_2) (* (Attributes|GetCurrentAttributes "NewEnumerator3") _defensemultiple_2)) (Variables|Initial|GetInitialDefense) (LocalVariables|GetArmorMagicDefense_L))))))

(fn CaculateDamageValue
  (params (Damage :type Float%20%28double-precision%29) (Defense :type Float%20%28double-precision%29))
  (return (* Damage (/ Damage Defense))))

(fn UpdateMaxStats
  (bind _keys (Utilities|Map|Keys (Variables|Stats|GetCurrentStats)))
  (for _array_element _keys
    (Stats|CalculationMaxStats _array_element)))