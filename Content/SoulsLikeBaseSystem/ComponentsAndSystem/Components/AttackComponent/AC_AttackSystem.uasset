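; Attack component that runs a character's attacks: melee, boss melee, spinning, ground smash, leaping long-range, magic projectiles and bullet traces.
; Attack events play a montage, message the owner on attack start and end, toggle interruptibility for some moves, and use notifies to fire AOEs, spells or jumps.
; Damage from weapon sphere traces, line traces, spawned AOE actors and projectiles is team-filtered.
; Leaps launch toward the target's predicted position.
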(event Custom|MagicSpell
  (params (SpawnTransform :type Transform) (Target :type Actor%20Object%20Reference) (DamageInfo :type S%20Damage%20Info%20Structure) (ProjectileBase :type BP%20Projectile%20Base%20Class%20Reference))
  ;[1 1 1] Attack Notify Helper
  ;;[1 1 1] magic
  (bind _returnvalue (Game|SpawnActorfromClass ProjectileBase SpawnTransform "Undefined" "MultiplyWithRoot" (Components|GetOwner) 1e+03 0.0 Target false 0))
  (EventDispatchers|AssignOnProjectileImpact _returnvalue (delegate Custom|OnProjectileHit))
  ;;;[1 1 1] Ignore the Spawn Actor collision
  (Collision|IgnoreActorwhenMoving (Actor|GetComponentbyClass (Components|GetOwner) "/Script/Engine.CapsuleComponent") _returnvalue true))

(event Custom|OnProjectileHit
  (params (OtherActor :type Actor%20Object%20Reference) (Hit :type Hit%20Result%20Structure))
  ;[1 1 1] Attack Notify Helper
  ;;[1 1 1] magic
  (bind _candamage (CallFunction|CheckTeam OtherActor))
  (if _candamage
    (Class|BIDamagable|TakeDamage(Message) OtherActor (stale Custom|MagicSpell DamageInfo) (Components|GetOwner) Hit))
  (Default|CallOnAttackEnd))

(event Custom|LongRangeMeleeAttack
  (params (AttackInfo :type S%20Attack%20Info%20Structure) (AoeRelativeSelfLocation :type Vector))
  (bind (_attacktarget _montage _damageinfo) (Utilities|Struct|BreakS_AttackInfo AttackInfo))
  (bind _returnvalue (Components|GetOwner))
  ;[1 1 1] LongRangeAttack
  (bind _mesh (CallFunction|AttackBase _attacktarget))
  (bind _notifyname (Animation|Montage|PlayMontage _mesh _montage)
    (:then
      (Class|BIDamagable|SetCanbeInterruptible(Message) _returnvalue false))
    (:OnCompleted
      (Class|BIEnemyAI|AttackEnd(Message) _returnvalue _attacktarget :!label _label)
      (Class|BIDamagable|SetCanbeInterruptible(Message) _returnvalue true))
    (:OnInterrupted
      (goto _label))
    (:OnNotifyBegin
      (switch name _notifyname
        (:Jump
          (CallFunction|JumptoAttackTarget _attacktarget))
        (:AOESlash
          (CallFunction|AOEDamage 3e+02 _damageinfo AoeRelativeSelfLocation))))))

(event Custom|OnAoeOverlapActor_Event
  (params (Actor :type Actor%20Object%20Reference) (Hit%20Result :type Hit%20Result%20Structure))
  ;[1 1 1] Attack Notify Helper
  ;;[1 1 1] AOEDamage
  (bind _candamage (CallFunction|CheckTeam Actor))
  (if _candamage
    (Class|BIDamagable|TakeDamage(Message) Actor (stale Custom|AOEDamage DamageInfo) (Components|GetOwner) Hit%20Result)))

(event Custom|SpiningMeleeAttack
  (params (AttackInfo :type S%20Attack%20Info%20Structure))
  (bind (_attacktarget _montage _damageinfo) (Utilities|Struct|BreakS_AttackInfo AttackInfo))
  (bind _returnvalue (Components|GetOwner))
  ;[1 1 1] SpiningMeleeAttack
  (bind _mesh (CallFunction|AttackBase _attacktarget))
  (bind _notifyname (Animation|Montage|PlayMontage _mesh _montage)
    (:then
      ;;[1 1 1] cannot be interrupted
      (Class|BIDamagable|SetCanbeInterruptible(Message) _returnvalue false))
    (:OnCompleted
      (Class|BIEnemyAI|AttackEnd(Message) _returnvalue _attacktarget :!label _label)
      (Class|BIDamagable|SetCanbeInterruptible(Message) _returnvalue true))
    (:OnInterrupted
      (goto _label))
    (:OnNotifyBegin
      (switch name _notifyname
        (:AOESlash
          (CallFunction|AOEDamage 3e+02 _damageinfo "0, 0, 0"))))))

(event Custom|AOEDamage
  (params (Radius :type Float%20%28single-precision%29) (DamageInfo :type S%20Damage%20Info%20Structure) (AoeRelativeSelfLocation :type Vector))
  (bind _returnvalue (Components|GetOwner))
  ;[1 1 1] Attack Notify Helper
  ;;[1 1 1] AOEDamage
  (bind _returnvalue_2 (Game|SpawnActorfromClass "/Game/SoulsLikeBaseSystem/ComponentsAndSystem/AOESystem/BP_AOE_Base.BP_AOE_Base_C" (Math|Transform|MakeTransform (+ (Transformation|GetActorLocation _returnvalue) (* AoeRelativeSelfLocation (Transformation|GetActorForwardVector _returnvalue))) "0, 0, 0" "1.000000,1.000000,1.000000") "Undefined" "MultiplyWithRoot" 0 true false (Variables|Default|GetAOE%20Draw%20Debug%20Type) (.AsPawn (Utilities|Casting|CastToPawn (Components|GetOwner)))))
  (Variables|/Game/SoulsLikeBaseSystem/ComponentsAndSystem/AOESystem/BP_AOE_Base.BP_AOE_Base_C|SetRadius _returnvalue_2 Radius)
  (EventDispatchers|AssignOnAoeOverlapActor _returnvalue_2 (delegate Custom|OnAoeOverlapActor_Event))
  (Default|Trigger _returnvalue_2))

(event Custom|ClearDamagedActors
  ;[1 1 1] Attack Notify Helper
  ;;[1 0 0.03636] MainWeaponTraceDamage  Based First Equiped Weapon. Need to set the weapon's slot and damage attributes,  Detect damage using the animation notifity state of the animation montage
  (Utilities|Array|Clear (Variables|Default|GetDamagedActors)))

(event Custom|PrimaryMeleeAttack
  (params (AttackInfo :type S%20Attack%20Info%20Structure))
  (bind (_attacktarget _montage) (Utilities|Struct|BreakS_AttackInfo AttackInfo))
  ;[1 1 1] PrimaryMeleeAttack
  (bind _mesh (CallFunction|AttackBase _attacktarget))
  (Animation|Montage|PlayMontage _mesh _montage
    (:OnCompleted
      _)
    (:OnInterrupted
      _))
  (Class|BIEnemyAI|AttackEnd(Message) (Components|GetOwner) _attacktarget))

(event Custom|BossPrimaryMeleeAttack
  (params (AttackInfo :type S%20Attack%20Info%20Structure))
  (bind (_attacktarget _montage) (Utilities|Struct|BreakS_AttackInfo AttackInfo))
  (bind _returnvalue (Components|GetOwner))
  ;[1 1 1] BossPrimaryMeleeAttack
  (bind _mesh (CallFunction|AttackBase _attacktarget))
  (Animation|Montage|PlayMontage _mesh _montage
    (:then
      ;;[1 1 1] Can not be interruptible
      (Class|BIDamagable|SetCanbeInterruptible(Message) _returnvalue false))
    (:OnCompleted
      (Class|BIEnemyAI|AttackEnd(Message) _returnvalue _attacktarget :!label _label)
      (Class|BIDamagable|SetCanbeInterruptible(Message) _returnvalue true))
    (:OnInterrupted
      (goto _label))))

(event Custom|JumpToAttackTarget
  (params (AttackTarget :type Actor%20Object%20Reference))
  (bind _returnvalue (Components|GetOwner))
  (bind _ascharacter (Utilities|Casting|CastToCharacter _returnvalue))
  ;[1 1 1] Attack Notify Helper
  ;;[1 1 1] jump to attack target location
  (bind _location (CallFunction|CalculateFutureActorLocation AttackTarget 1.0))
  (bind _outlaunchvelocity (Game|SuggestProjectileVelocityCustomArc (Transformation|GetActorLocation (Components|GetOwner)) (Math|Vector|MakeVector (.x _location) (.y _location) (+ (.z _location) 1e+02)) 0.0 (Math|Float|Lerp 0.8 0.95 (Math|Float|Clamp(Float) (Math|Float|NormalizetoRange (Transformation|GetDistanceTo AttackTarget (Components|GetOwner)) 4e+02 8e+02)))))
  (Character|LaunchCharacter _ascharacter _outlaunchvelocity true true)
  (EventDispatchers|AssignLandedDelegate _ascharacter (delegate Custom|OnLand)))

(event Custom|WeaponTraceDamage
  ;[1 1 1] Attack Notify Helper
  ;;[1 0 0.03636] MainWeaponTraceDamage  Based First Equiped Weapon. Need to set the weapon's slot and damage attributes,  Detect damage using the animation notifity state of the animation montage
  (if (Variables|Default|GetCanDoWeaponTrace)
    (bind _mainweapon (Class|BIDamagable|GetMainWeapon(Message) (Components|GetOwner)))
    (Utilities|IsValid _mainweapon
      (:Is%20Valid
        (bind (_outhits _returnvalue) (Collision|MultiSphereTraceForObjects (Transformation|GetSocketLocation (Variables|/Game/SoulsLikeBaseSystem/ComponentsAndSystem/WeaponSystem/BP_Weapon_Base.BP_Weapon_Base_C|GetMesh _mainweapon) "Start") (Transformation|GetSocketLocation (Variables|/Game/SoulsLikeBaseSystem/ComponentsAndSystem/WeaponSystem/BP_Weapon_Base.BP_Weapon_Base_C|GetMesh _mainweapon) "End") (Variables|/Game/SoulsLikeBaseSystem/ComponentsAndSystem/WeaponSystem/BP_Weapon_Base.BP_Weapon_Base_C|GetRadius _mainweapon) (Utilities|Array|MakeArray "ObjectTypeQuery3") false (Utilities|Array|MakeArray (Components|GetOwner)) (Variables|Default|GetMeleeWeaponTraceDebug)))
        (if _returnvalue
          (CallFunction|DamageAllNonTeamMembers _outhits (Variables|/Game/SoulsLikeBaseSystem/ComponentsAndSystem/WeaponSystem/BP_Weapon_Base.BP_Weapon_Base_C|GetDamageInfo _mainweapon))))
      (:Is%20Not%20Valid
        (Development|PrintString "Main Weapon None")))))

(event Custom|BasicMagicSpell
  (params (AttackInfo :type S%20Attack%20Info%20Structure) (ProjectileBase :type BP%20Projectile%20Base%20Class%20Reference))
  (bind (_attacktarget _montage _damageinfo) (Utilities|Struct|BreakS_AttackInfo AttackInfo))
  ;[1 1 1] BasicMagicSpell
  (bind _mesh (CallFunction|AttackBase _attacktarget))
  (bind _notifyname (Animation|Montage|PlayMontage _mesh _montage)
    (:OnCompleted
      (Class|BIEnemyAI|AttackEnd(Message) (Components|GetOwner) _attacktarget :!label _label))
    (:OnInterrupted
      (goto _label))
    (:OnNotifyBegin
      (switch name _notifyname
        (:Fire
          (CallFunction|MagicSpell (Math|Transform|MakeTransform (Transformation|GetSocketLocation _mesh (Variables|Default|GetMagicSpawnSocketName)) "0, 0, 0" "1.000000,1.000000,1.000000") _attacktarget _damageinfo ProjectileBase))))))

(event Custom|BarrageMagicAttack
  (params (AttackInfo :type S%20Attack%20Info%20Structure) (ProjectileBase :type BP%20Projectile%20Base%20Class%20Reference))
  (bind (_attacktarget _montage _damageinfo) (Utilities|Struct|BreakS_AttackInfo AttackInfo))
  (bind _returnvalue (Components|GetOwner))
  ;[1 1 1] BarrageMagicAttack
  (bind _mesh (CallFunction|AttackBase _attacktarget))
  (bind _notifyname (Animation|Montage|PlayMontage _mesh _montage)
    (:OnCompleted
      (Class|BIEnemyAI|AttackEnd(Message) _returnvalue _attacktarget :!label _label)
      ;;[1 1 1] cannot be interrupted
      (Class|BIDamagable|SetCanbeInterruptible(Message) _returnvalue true))
    (:OnInterrupted
      (goto _label))
    (:OnNotifyBegin
      (switch name _notifyname
        (:Fire
          (CallFunction|MagicSpell (Math|Transform|MakeTransform (Transformation|GetSocketLocation _mesh (Variables|Default|GetMagicSpawnSocketName)) (Math|Rotator|FindLookatRotation (Transformation|GetActorLocation (Components|GetOwner)) (+ (Transformation|GetActorLocation _attacktarget) (Math|Vector|MakeVector 0.0 (Math|Random|RandomFloatinRange -3e+02 3e+02) 0.0))) "1.000000,1.000000,1.000000") 0 _damageinfo ProjectileBase)
          (Class|BIDamagable|SetCanbeInterruptible(Message) _returnvalue false))))))

(event Custom|GroundSmashAOE
  (params (AttackInfo :type S%20Attack%20Info%20Structure) (Radius :type Float%20%28single-precision%29) (AoeRelativeSelfLocation :type Vector))
  (bind (_attacktarget _montage _damageinfo) (Utilities|Struct|BreakS_AttackInfo AttackInfo))
  (bind _returnvalue (Components|GetOwner))
  (bind (_damageamount _weapontype) (Utilities|Struct|BreakS_DamageInfo _damageinfo))
  ;[1 1 1] GroundSmash
  (bind _mesh (CallFunction|AttackBase _attacktarget))
  (bind _notifyname (Animation|Montage|PlayMontage _mesh _montage)
    (:then
      ;;[1 1 1] cannot be interrupted
      (Class|BIDamagable|SetCanbeInterruptible(Message) _returnvalue false))
    (:OnCompleted
      (Class|BIEnemyAI|AttackEnd(Message) _returnvalue _attacktarget :!label _label)
      ;;[1 1 1] can be interrupted
      (Class|BIDamagable|SetCanbeInterruptible(Message) _returnvalue true))
    (:OnInterrupted
      (goto _label))
    (:OnNotifyBegin
      (switch name _notifyname
        (:Smash
          (CallFunction|AOEDamage Radius (Utilities|Struct|MakeS_DamageInfo _damageamount _weapontype) AoeRelativeSelfLocation))))))

(event Custom|OnLand
  (params (Hit :type Hit%20Result%20Structure%20%28by%20ref%29))
  (bind _returnvalue (Components|GetOwner))
  (bind _ascharacter (Utilities|Casting|CastToCharacter _returnvalue))
  ;[1 1 1] Attack Notify Helper
  ;;[1 1 1] jump to attack target location
  (EventDispatchers|UnbindEventfromLandedDelegate _ascharacter (delegate Custom|OnLand))
  (Components|Movement|StopMovementImmediately (Variables|/Script/Engine.Character|GetCharacterMovement _ascharacter)))

(event Custom|FireBullet
  (params (TraceStart :type Vector) (TraceEnd :type Vector) (DamageInfo :type S%20Damage%20Info%20Structure))
  ;[1 1 1] Attack Notify Helper
  ;;[1 1 1] FireBullet
  (bind (_outhits _returnvalue) (Class|KismetSystemLibrary|LineTraceMultiforObjects TraceStart TraceEnd (Utilities|Array|MakeArray "ObjectTypeQuery3") false (Utilities|Array|MakeArray (Components|GetOwner)) (Variables|Default|GetShootDrawDebugType) true))
  (if _returnvalue
    (CallFunction|DamageFirstNonTeamMember _outhits DamageInfo)))

(event EventBeginPlay)

(event EventTick
  (params (DeltaSeconds :type Float%20%28single-precision%29)))

(fn DamageAllNonTeamMembers
  (params (Hits :type Array%20of%20Hit%20Result%20Structures) (DamageInfo :type S%20Damage%20Info%20Structure))
  (for _array_element Hits
    (bind _teamnumber (Class|BIDamagable|GetTeamNumber(Message) (.HitActor (Collision|BreakHitResult _array_element))))
    (bind _teamnumber_2 (Class|BIDamagable|GetTeamNumber(Message) (Components|GetOwner)))
    (if (and (!= _teamnumber_2 _teamnumber) (not (Utilities|Array|ContainsItem (Variables|Default|GetDamagedActors) (.HitActor (Collision|BreakHitResult _array_element)))))
      (Class|BIDamagable|TakeDamage(Message) (.HitActor (Collision|BreakHitResult _array_element)) DamageInfo (Components|GetOwner) _array_element)
      (Utilities|Array|AddUnique (Variables|Default|GetDamagedActors) (.HitActor (Collision|BreakHitResult _array_element)))))
  (return (Variables|Default|GetDamagedActors)))

(fn DamageFirstNonTeamMember
  (params (Hits :type Array%20of%20Hit%20Result%20Structures) (DamageInfo :type S%20Damage%20Info%20Structure))
  (bind _array_element (Utilities|Array|ForEachLoopwithBreak Hits :!label _label)
    (:LoopBody
      (bind _candamage (CallFunction|CheckTeam (.HitActor (Collision|BreakHitResult _array_element))))
      (if _candamage
        (Class|BIDamagable|TakeDamage(Message) (.HitActor (Collision|BreakHitResult _array_element)) DamageInfo (Components|GetOwner) _array_element)
        (Utilities|FlowControl|Sequence
          (:then_0
            (goto _label Break))
          (:then_1
            (return (.HitActor (Collision|BreakHitResult _array_element)))))))))

(fn AttackBase
  (params (AttackTarget :type Actor%20Object%20Reference))
  (bind _returnvalue (Components|GetOwner))
  (Class|BIEnemyAI|Attack(Message) _returnvalue AttackTarget)
  (bind _ascharacter (Utilities|Casting|CastToCharacter _returnvalue)
    (:then
      _)
    (:CastFailed
      _))
  (return (Variables|/Script/Engine.Character|GetMesh _ascharacter)))

(fn CalculateFutureActorLocation
  (params (Actor :type Actor%20Object%20Reference) (Time :type Float%20%28double-precision%29))
  (bind _returnvalue (Transformation|GetVelocity Actor))
  (if (Utilities|Operators|NotEqual(!=) :A _returnvalue :ErrorTolerance 0.1)
    (return (+ (Transformation|GetActorLocation Actor) (* (* _returnvalue "1.000000,1.000000,0.000000") Time)))
    (else
      (return (Transformation|GetActorLocation Actor)))))

(fn CheckTeam
  (params (OtherActor :type Actor%20Object%20Reference))
  (bind _teamnumber (Class|BIDamagable|GetTeamNumber(Message) OtherActor))
  (bind _teamnumber_2 (Class|BIDamagable|GetTeamNumber(Message) (Components|GetOwner)))
  (return (!= _teamnumber_2 _teamnumber)))