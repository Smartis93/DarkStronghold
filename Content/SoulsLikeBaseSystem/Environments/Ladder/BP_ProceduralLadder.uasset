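; Procedural climbable ladder actor that registers itself on BP_PlayerTesi while the player overlaps its entry box.
; The construction script scales the side rails to LadderHeight, adds instanced rungs at LadderGap spacing with optional interval screws, then places end pieces and exit components at the top.
; Overlapping the exit box in a specific combat state changes that state, restores walking and teleports the player to the Box transform.
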(event OnComponentBeginOverlap(EnterBpx)
  (params (OverlappedComponent :type Primitive%20Component%20Object%20Reference) (OtherActor :type Actor%20Object%20Reference) (OtherComp :type Primitive%20Component%20Object%20Reference) (OtherBodyIndex :type Integer) (bFromSweep :type Boolean) (SweepResult :type Hit%20Result%20Structure%20%28by%20ref%29))
  (bind _asbp_player_tesi (Utilities|Casting|CastToBP_PlayerTesi OtherActor))
  (Variables|/Game/MicheleTesi/Blueprint/Player/BP_PlayerTesi.BP_PlayerTesi_C|SetLadderRef _asbp_player_tesi self))

(event OnComponentEndOverlap(EnterBpx)
  (params (OverlappedComponent :type Primitive%20Component%20Object%20Reference) (OtherActor :type Actor%20Object%20Reference) (OtherComp :type Primitive%20Component%20Object%20Reference) (OtherBodyIndex :type Integer))
  (bind _asbp_player_tesi (Utilities|Casting|CastToBP_PlayerTesi OtherActor))
  (Variables|/Game/MicheleTesi/Blueprint/Player/BP_PlayerTesi.BP_PlayerTesi_C|SetLadderRef _asbp_player_tesi 0))

(event OnComponentBeginOverlap(ExitBox)
  (params (OverlappedComponent :type Primitive%20Component%20Object%20Reference) (OtherActor :type Actor%20Object%20Reference) (OtherComp :type Primitive%20Component%20Object%20Reference) (OtherBodyIndex :type Integer) (bFromSweep :type Boolean) (SweepResult :type Hit%20Result%20Structure%20%28by%20ref%29))
  (bind _box (Variables|Default|GetBox))
  (bind _returnvalue (Transformation|GetWorldTransform _box))
  (bind _asbp_player_tesi (Utilities|Casting|CastToBP_PlayerTesi OtherActor))
  (bind _ac_combat (Variables|/Game/MicheleTesi/Blueprint/Player/BP_PlayerTesi.BP_PlayerTesi_C|GetAC_Combat _asbp_player_tesi)
    (:then
      (if (Utilities|Enum|Equal(Enum) "NewEnumerator6" (Variables|/Game/MicheleTesi/Blueprint/Player/AC_Combat.AC_Combat_C|GetCurrent%20State _ac_combat))
        (Default|ChangeState _ac_combat "NewEnumerator0")
        (Pawn|Components|CharacterMovement|SetMovementMode (Variables|/Script/Engine.Character|GetCharacterMovement _asbp_player_tesi) "MOVE_Walking" 0)
        (Transformation|SetActorLocationAndRotation _asbp_player_tesi (.location _returnvalue) (.rotation _returnvalue) false true)))
    (:else)))

(event EventBeginPlay)

(event Collision|EventActorBeginOverlap
  (params (OtherActor :type Actor%20Object%20Reference)))

(event EventTick
  (params (DeltaSeconds :type Float%20%28single-precision%29)))

(fn ConstructionScript
  (Transformation|SetRelativeScale3D (Variables|Default|GetLeftLadder) (Math|Vector|MakeVector 0.1 0.1 (Variables|Default|GetLadder%20Height)))
  (while (< (Variables|Default|GetCompare%20Height) (* (Variables|Default|GetLadder%20Height) 1e+02))
    (Utilities|AddBarsandScrews))
  (Utilities|FlowControl|Sequence
    (:then_0
      (CallFunction|SetLadderEndPieces))
    (:then_1
      (CallFunction|SetLadderExitArea))))

(fn SetLadderEndPieces
  (bind _ladder_height (Variables|Default|GetLadder%20Height))
  (bind _end_piece_type (Variables|Default|GetEnd%20Piece%20Type))
  (bind _returnvalue (* _ladder_height 1e+02))
  (bind _returnvalue_2 (Utilities|Select :Index _end_piece_type :NewEnumerator0 0 :NewEnumerator1 0 :NewEnumerator2 "/Game/SoulsLikeBaseSystem/Environments/Ladder/EndPieces/LadderEndCurve.LadderEndCurve"))
  (Transformation|SetRelativeLocation (Variables|Default|GetLeftPoleEnd) (Math|Vector|MakeVector 0.0 -3e+01 _returnvalue) false false)
  (Transformation|SetRelativeLocation (Variables|Default|GetRightPoleEnd) (Math|Vector|MakeVector 0.0 3e+01 _returnvalue) false false)
  (Components|StaticMesh|SetStaticMesh (Variables|Default|GetLeftPoleEnd) _returnvalue_2)
  (Components|StaticMesh|SetStaticMesh (Variables|Default|GetRightPoleEnd) _returnvalue_2))

(fn SetLadderExitArea
  (bind _ladder_height (Variables|Default|GetLadder%20Height))
  (bind _returnvalue (* _ladder_height 1e+02))
  (Transformation|SetRelativeLocation (Variables|Default|GetExitBox) (Math|Vector|MakeVector -3e+01 0.0 (+ _returnvalue (Variables|Default|GetExit%20Box%20Offset))) false false)
  (Transformation|SetRelativeLocation (Variables|Default|GetLadderExitPosition) (Math|Vector|MakeVector 0.0 0.0 _returnvalue) false false))