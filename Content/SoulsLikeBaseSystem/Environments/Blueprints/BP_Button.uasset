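; BP_Button is an environment button the player can press to open a linked door.
; Its Box overlap registers the button on BP_PlayerTesi on entry and clears that reference on exit.
; PressButton calls OpenDoorWithButton on the DoorSelect reference, then sets the Box to visible in game.
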(event OnComponentBeginOverlap(Box)
  (params (OverlappedComponent :type Primitive%20Component%20Object%20Reference) (OtherActor :type Actor%20Object%20Reference) (OtherComp :type Primitive%20Component%20Object%20Reference) (OtherBodyIndex :type Integer) (bFromSweep :type Boolean) (SweepResult :type Hit%20Result%20Structure%20%28by%20ref%29))
  (bind _asbp_player_tesi (Utilities|Casting|CastToBP_PlayerTesi OtherActor))
  (Variables|/Game/MicheleTesi/Blueprint/Player/BP_PlayerTesi.BP_PlayerTesi_C|SetButton _asbp_player_tesi self))

(event OnComponentEndOverlap(Box)
  (params (OverlappedComponent :type Primitive%20Component%20Object%20Reference) (OtherActor :type Actor%20Object%20Reference) (OtherComp :type Primitive%20Component%20Object%20Reference) (OtherBodyIndex :type Integer))
  (bind _asbp_player_tesi (Utilities|Casting|CastToBP_PlayerTesi OtherActor))
  (Variables|/Game/MicheleTesi/Blueprint/Player/BP_PlayerTesi.BP_PlayerTesi_C|SetButton _asbp_player_tesi 0))

(event Custom|PressButton
  (Default|OpenDoorwithButton (Variables|Default|GetDoorSelect))
  (Development|SetHiddeninGame (Variables|Default|GetBox) false false))

(fn ConstructionScript)