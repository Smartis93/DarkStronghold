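; BP_Door is an interactable door that swings open or shut each time it is triggered.
; Overlapping InteractionBox registers the door as BP_PlayerTesi's Door reference, and leaving the box clears it.
; Interact and DoorInteraction share one toggle on DoorOpen that plays or reverses OpenCloseTimeline.
; The timeline's DoorAngle drives the Door's relative rotation, though only the Play call shows an update handler.
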(event OnComponentBeginOverlap(InteractionBox)
  (params (OverlappedComponent :type Primitive%20Component%20Object%20Reference) (OtherActor :type Actor%20Object%20Reference) (OtherComp :type Primitive%20Component%20Object%20Reference) (OtherBodyIndex :type Integer) (bFromSweep :type Boolean) (SweepResult :type Hit%20Result%20Structure%20%28by%20ref%29))
  (bind _asbp_player_tesi (Utilities|Casting|CastToBP_PlayerTesi OtherActor))
  (Variables|/Game/MicheleTesi/Blueprint/Player/BP_PlayerTesi.BP_PlayerTesi_C|SetDoor _asbp_player_tesi self))

(event OnComponentEndOverlap(InteractionBox)
  (params (OverlappedComponent :type Primitive%20Component%20Object%20Reference) (OtherActor :type Actor%20Object%20Reference) (OtherComp :type Primitive%20Component%20Object%20Reference) (OtherBodyIndex :type Integer))
  (bind _asbp_player_tesi (Utilities|Casting|CastToBP_PlayerTesi OtherActor))
  (Variables|/Game/MicheleTesi/Blueprint/Player/BP_PlayerTesi.BP_PlayerTesi_C|SetDoor _asbp_player_tesi 0))

(event Custom|Door%20Interaction
  (if (not (Variables|Default|GetDoorOpen?))
    (Variables|Default|SetDoorOpen? true)
    (bind _door_angle (Timeline|OpenClose%20Timeline Play)
      (:Update
        (Transformation|SetRelativeRotation (Variables|Default|GetDoor) (Math|Rotator|MakeRotator 0.0 0.0 _door_angle) false false)))
    (else
      (Variables|Default|SetDoorOpen? false)
      (Timeline|OpenClose%20Timeline Reverse))))

(event EventInteract
  (if (not (Variables|Default|GetDoorOpen?))
    (Variables|Default|SetDoorOpen? true)
    (bind _door_angle (Timeline|OpenClose%20Timeline Play)
      (:Update
        (Transformation|SetRelativeRotation (Variables|Default|GetDoor) (Math|Rotator|MakeRotator 0.0 0.0 _door_angle) false false)))
    (else
      (Variables|Default|SetDoorOpen? false)
      (Timeline|OpenClose%20Timeline Reverse))))

(fn ConstructionScript
  (|CallParentFunction))