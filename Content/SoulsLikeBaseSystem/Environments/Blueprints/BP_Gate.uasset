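; BP_Gate is a one-way double gate that opens only when GateInteraction is called from the right side.
; Two trigger overlaps set DoorState, resetting it to Neutral on exit.
; From the right side, it plays a sound, swings both leaves via timelines (the left started from the right's update) and disables wrong-side trigger collision.
; From the wrong side, it shows a notification widget, with a delayed reference reset limiting repeats.
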(event OnComponentBeginOverlap(RightSideCollider)
  (params (OverlappedComponent :type Primitive%20Component%20Object%20Reference) (OtherActor :type Actor%20Object%20Reference) (OtherComp :type Primitive%20Component%20Object%20Reference) (OtherBodyIndex :type Integer) (bFromSweep :type Boolean) (SweepResult :type Hit%20Result%20Structure%20%28by%20ref%29))
  (Variables|Default|SetDoorState "NewEnumerator1"))

(event OnComponentEndOverlap(RightSideCollider)
  (params (OverlappedComponent :type Primitive%20Component%20Object%20Reference) (OtherActor :type Actor%20Object%20Reference) (OtherComp :type Primitive%20Component%20Object%20Reference) (OtherBodyIndex :type Integer))
  (Variables|Default|SetDoorState "NewEnumerator0"))

(event OnComponentBeginOverlap(WrongSideTrigger)
  (params (OverlappedComponent :type Primitive%20Component%20Object%20Reference) (OtherActor :type Actor%20Object%20Reference) (OtherComp :type Primitive%20Component%20Object%20Reference) (OtherBodyIndex :type Integer) (bFromSweep :type Boolean) (SweepResult :type Hit%20Result%20Structure%20%28by%20ref%29))
  (Variables|Default|SetDoorState "NewEnumerator2"))

(event OnComponentEndOverlap(WrongSideTrigger)
  (params (OverlappedComponent :type Primitive%20Component%20Object%20Reference) (OtherActor :type Actor%20Object%20Reference) (OtherComp :type Primitive%20Component%20Object%20Reference) (OtherBodyIndex :type Integer))
  (Variables|Default|SetDoorState "NewEnumerator0"))

(event Custom|GateInteraction
  (switch Utilities|FlowControl|Switch|SwitchonE_DoorState (Variables|Default|GetDoorState)
    (:NewEnumerator1
      (Audio|PlaySoundatLocation "/Engine/VREditor/Sounds/UI/Dockable_Window_Open.Dockable_Window_Open" (Transformation|GetActorLocation) "0, 0, 0" 1.0 1.0 0.0 0 0 0 0)
      (bind _float (Timeline|RightDoor Play)
        (:Update
          (Transformation|SetRelativeRotation (Variables|Default|GetRightSide) (Math|Rotator|MakeRotator 0.0 0.0 (Math|Float|Lerp 1.8e+02 3e+02 _float)) false false)
          (bind _float_2 (Timeline|LeftDoor Play)
            (:Update
              (Transformation|SetRelativeRotation (Variables|Default|GetLeftSide) (Math|Rotator|MakeRotator 0.0 0.0 (Math|Float|Lerp 0.0 -1.2e+02 _float_2)) false false)
              (Collision|SetCollisionEnabled (Variables|Default|GetWrongSideTrigger) "NoCollision"))))))
    (:NewEnumerator2
      (Utilities|IsValid (Variables|Default|GetNotificationWidget)
        (:Is%20Not%20Valid
          (bind _returnvalue (UserInterface|CreateWidget "/Game/SoulsLikeBaseSystem/Widget/W_Notification.W_Notification_C" 0 "Wrong Side.."))
          (bind _output_get (Variables|Default|SetNotificationWidget _returnvalue))
          (UserInterface|Viewport|AddtoViewport _output_get 0)
          (Utilities|FlowControl|Delay 3.5)
          (Variables|Default|SetNotificationWidget 0))))))

(fn ConstructionScript)